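; AI controller for BP_BaseEnemy pawns that chases the player's wizard and attacks on reaching it.
; On pawn begin play it caches the enemy's attack range and charge time, waits a wake-up delay, then moves to the player using that range as acceptance radius.
; A successful move triggers a charge, delay and attack.
; Move completion restarts the chase, polling briefly until the enemy is no longer stunned.
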(event `self.ReceiveBeginPlay`
  (`parent.ReceiveBeginPlay`))

(event `self.OnPawnBeginPlay`
  (`parent.OnPawnBeginPlay`)
  (bind _asbp_wizard_character (cast `/Game/BP/BP_WizardCharacter` (`GameplayStatics.GetPlayerPawn` 0)))
  (set `self.As BP Wizard Character 2` _asbp_wizard_character)
  (add `self.ReceiveMoveCompleted` (delegate `MovementCompleted`))
  (bind _asbp_base_enemy (cast `/Game/BP/Enemies/BP_BaseEnemy` (`self.K2_GetPawn`)))
  (set `self.AttackRange` (`/Game/BP/Enemies/BP_BaseEnemy.AttackRange` _asbp_base_enemy))
  (set `self.AttackChargeTime` (`/Game/BP/Enemies/BP_BaseEnemy.AttackChargeTime` _asbp_base_enemy))
  (`KismetSystemLibrary.Delay` (`self.WakeUpDuration`))
  (`self.MoveToPlayer`))

(event `MovementCompleted` :!signature `self.ReceiveMoveCompleted`
  (params (RequestID :type "AIRequestID Structure") (Result :type "EPathFollowingResult Enum" :default "Success"))
  (switch `EPathFollowingResult` Result
    (:`Success`
      (`self.ChargeAttack`)
      (`KismetSystemLibrary.Delay` (`self.AttackChargeTime`))
      (`self.InitiateAttack`))
    (:`Blocked`
      _)
    (:`OffPath`
      _)
    (:`Aborted`
      _)
    (:`Invalid`
      _))
  (`KismetSystemLibrary.Delay` 0.05 :!label _label)
  (bind _asbp_base_enemy (cast `/Game/BP/Enemies/BP_BaseEnemy` (`self.K2_GetPawn`)))
  (bind _returnvalue (`BaseCharacter.GetStunned` _asbp_base_enemy))
  (if _returnvalue
    (goto _label)
    (else
      (`self.MoveToPlayer`))))

(fn `Attack`
  (`parent.Attack`))

(fn `ChargeAttack`
  (bind _asbp_base_enemy (cast `/Game/BP/Enemies/BP_BaseEnemy` (`self.K2_GetPawn`)))
  (`/Game/BP/Enemies/BP_BaseEnemy.ChargeAttack` _asbp_base_enemy))

(fn `MoveToPlayer`
  (returns (result :type "EPathFollowingRequestResult Enum"))
  (bind _returnvalue (`self.MoveToActor` (`self.As BP Wizard Character 2`) (`self.AttackRange`) true true true null))
  (return _returnvalue))

(fn `UserConstructionScript`
  (`parent.UserConstructionScript`))