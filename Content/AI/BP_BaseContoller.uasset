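; Base AI controller for BP_BaseEnemy pawns that handles attack requests and stun reactions.
; OnPawnBeginPlay binds to the controlled enemy's Stunned event, which stops movement when fired.
; InitiateAttack checks that the enemy is not stunned, then calls Attack, which forwards the attack to the pawn.
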(event `self.ReceiveBeginPlay`)

(event `OnPawnBeginPlay`
  (bind _asbp_base_enemy (cast `/Game/Enemies/BP_BaseEnemy` (`self.K2_GetPawn`)))
  (add `/Game/Enemies/BP_BaseEnemy.Stunned` _asbp_base_enemy (delegate `OnStunned`)))

(event `OnStunned`
  (`self.StopMovement`))

(fn `Attack`
  (bind _asbp_base_enemy (cast `/Game/Enemies/BP_BaseEnemy` (`self.K2_GetPawn`)))
  (`/Game/Enemies/BP_BaseEnemy.Attack` _asbp_base_enemy))

(fn `InitiateAttack`
  (bind _asbp_base_enemy (cast `/Game/Enemies/BP_BaseEnemy` (`self.K2_GetPawn`)))
  (bind _returnvalue (`BaseCharacter.GetStunned` _asbp_base_enemy))
  (if (not _returnvalue)
    (`self.Attack`)))

(fn `UserConstructionScript`)