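; Ranged enemy Blueprint whose attack shoots a projectile straight at player 0's pawn.
; Attack spawns the Projectile class at the enemy's location, scaled down and rotated toward the player, passing the enemy's instigator as owner and instigator.
; It casts the result to BaseProjectile and calls FireInDirection with the normalized vector to the player's current position.
; The event graph holds only disabled stubs, so Attack is triggered outside these graphs.
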(fn `Attack`
  (bind _returnvalue (`self.GetInstigator`))
  (bind _returnvalue_2 (`self.K2_GetActorLocation`))
  (bind _returnvalue_3 (- (`self.K2_GetActorLocation` (`GameplayStatics.GetPlayerPawn` 0)) _returnvalue_2))
  (bind _returnvalue_4 (`|SpawnActorFromClass` (`self.Projectile`) (`KismetMathLibrary.MakeTransform` _returnvalue_2 (`KismetMathLibrary.Conv_VectorToRotator` _returnvalue_3) (0.75 0.75 0.75)) "Undefined" "OverrideRootScale" _returnvalue _returnvalue))
  (bind _asbase_projectile (cast `BaseProjectile` _returnvalue_4))
  (`BaseProjectile.FireInDirection` _asbase_projectile (`KismetMathLibrary.Normal` _returnvalue_3)))

(fn `UserConstructionScript`
  (`parent.UserConstructionScript`))