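; BP_BaseEnemy is a base enemy pawn with a health bar, a score reward and empty Attack and ChargeAttack functions.
; On BeginPlay it notifies its BP_BaseContoller, and each Tick it sets the Healthbar widget to current health over starting health.
; Stun events are relayed through CallStunned, and on death it adds ScoreReward to its Spawner's score if that spawner is valid.
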(event `self.ReceiveBeginPlay`
  (bind _asbp_base_contoller (cast `/Game/AI/BP_BaseContoller` (`self.GetController`)))
  (`/Game/AI/BP_BaseContoller.OnPawnBeginPlay` _asbp_base_contoller))

(event `self.ReceiveTick`
  (params (DeltaSeconds :type "Float (single-precision)"))
  (bind _ashealthbar (cast `/Game/UI/Healthbar` (`WidgetComponent.GetWidget` (`self.Healthbar`))))
  (bind _returnvalue (`self.GetHealth`))
  (bind _returnvalue_2 (`self.GetStartHealth`))
  (`/Game/UI/Healthbar.SetPercentage` _ashealthbar (/ _returnvalue _returnvalue_2)))

(event `self.OnStunned`
  (`self.Stunned`))

(event `self.OnDeath`
  (bind _spawner (`self.Spawner`))
  (if (`KismetSystemLibrary.IsValid` _spawner)
    (`/Game/Enemies/Spawner.AddScore` _spawner (`self.ScoreReward`))))

(fn `Attack`)

(fn `ChargeAttack`)

(fn `UserConstructionScript`)