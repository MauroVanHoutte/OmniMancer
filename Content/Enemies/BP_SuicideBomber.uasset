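; BP_SuicideBomber is an enemy that damages wizard characters around it with a one-shot explosion and destroys itself.
; On BeginPlay it scales ExplosionZone into a flattened area sized by ExplosionRadius.
; ChargeAttack reveals that zone in game as a visible warning.
; Attack applies spell damage to every overlapping BP_WizardCharacter, then destroys the bomber even if nothing was hit.
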(event `self.ReceiveBeginPlay`
  (bind _explosionradius (`self.ExplosionRadius`))
  (`parent.ReceiveBeginPlay`)
  (`SceneComponent.SetRelativeScale3D` (`self.ExplosionZone`) (`KismetMathLibrary.MakeVector` _explosionradius _explosionradius 0.2)))

(fn `Attack`
  (bind _overlappingactors (`PrimitiveComponent.GetOverlappingActors` (`self.ExplosionZone`) "/Game/BP_WizardCharacter.BP_WizardCharacter_C"))
  (if (> (`KismetArrayLibrary.Array_Length` _overlappingactors) 0)
    (for _array_element _overlappingactors
      (bind _asbp_wizard_character (cast `/Game/BP_WizardCharacter` _array_element))
      (`self.TakeSpellDamage` _asbp_wizard_character (`self.Damage`))))
  (`self.K2_DestroyActor`))

(fn `ChargeAttack`
  (`SceneComponent.SetHiddenInGame` (`self.ExplosionZone`) false false))

(fn `UserConstructionScript`
  (`parent.UserConstructionScript`))