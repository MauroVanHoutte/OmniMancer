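; BP_MortarProjectile is an enemy mortar projectile that leaves a BP_IceZone hazard where it explodes.
; SetParameter stores the zone's lifespan, scale, burn and slow settings on the projectile.
; SpawnExplosion traces a short distance down from the given location with the InvisibleWall profile, spawns the zone at the trace's hit location, and passes those stored settings to it.
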(event `self.SpawnExplosion`
  (params (location :type "Vector Structure (by ref)"))
  (bind _outhit (`KismetSystemLibrary.LineTraceSingleByProfile` location (- location (0.0 0.0 100.0)) "InvisibleWall"))
  (bind _returnvalue (`|SpawnActorFromClass` "/Game/BP/Spells/BP_IceZone.BP_IceZone_C" (`KismetMathLibrary.MakeTransform` (`.Location` (`GameplayStatics.BreakHitResult` _outhit))) "Undefined" "OverrideRootScale" self self))
  (`/Game/BP/Spells/BP_IceZone.Set Parameters` _returnvalue (`self.Lifespan`) (`self.Zone Scale`) (`self.Apply Burn`) (`self.Burn Tick Damage`) (`self.Burn Tick Interval`) (`self.Duration`) (`self.Apply Slow`) (`self.Slow Value`)))

(fn `Set Parameter`
  (params (Lifespan :type "Float (double-precision)") (ZoneScale :type "Vector Structure") (ApplyBurn :type Boolean) (BurnTickDamage :type "Float (double-precision)") (BurnTickInterval :type "Float (double-precision)") (Duration :type "Float (double-precision)") (ApplySlow :type Boolean) (SlowValue :type "Float (double-precision)"))
  (set `self.Lifespan` Lifespan)
  (set `self.Zone Scale` ZoneScale)
  (set `self.Apply Burn` ApplyBurn)
  (set `self.Burn Tick Damage` BurnTickDamage)
  (set `self.Burn Tick Interval` BurnTickInterval)
  (set `self.Duration` Duration)
  (set `self.Apply Slow` ApplySlow)
  (set `self.Slow Value` SlowValue))

(fn `UserConstructionScript`)