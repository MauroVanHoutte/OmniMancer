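; BP_BossEnemy is an enemy Blueprint for bosses that hands its attacks to a Moveset.
; Attack executes a move on the target and starts a cooldown timer if the result is valid, otherwise it signals attack completion.
; CanAttack combines the parent check with that timer being inactive.
; Trigger hits and repeat-hit checks are forwarded to the Moveset, and an affiliation component is exposed.
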(event `AttackTimerCompleted`)

(event `HitTriggerInterface.OnTriggered`
  (params (TriggeringActor :type "Actor Object Reference") (ColliderComponent :type "PrimitiveComponent Object Reference"))
  (`MovesetComponent.OnHitTriggered` (`self.Moveset`) TriggeringActor ColliderComponent))

(fn `Attack`
  (params (Target :type "Actor Object Reference"))
  (bind _returnvalue (`MovesetComponent.ExecuteAttack` (`self.Moveset`) Target))
  (if (`KismetSystemLibrary.IsValid` _returnvalue)
    (bind _returnvalue_2 (`KismetSystemLibrary.K2_SetTimerDelegate` (`|CreateDelegate` :!event `AttackTimerCompleted`) (`self.AttackCooldown_0`)))
    (set `self.AttackTimer` _returnvalue_2)
    (else
      (`self.AttackComplete`))))

(fn `CanAttack`
  (params (Target :type "Actor Object Reference"))
  (returns (CanAttack :type Boolean))
  (bind _canattack (`parent.CanAttack` Target))
  (return (and _canattack (not (`KismetSystemLibrary.K2_IsTimerActiveHandle` (`self.AttackTimer`))))))

(fn `GetAffiliation`
  (returns (ReturnValue :type "AffiliationComponent Object Reference"))
  (return (`self.AffiliationComponent`)))

(fn `InterruptAttack`
  (`parent.InterruptAttack`))

(fn `IsAttackInterruptable`
  (returns (Interruptable :type Boolean))
  (bind _interruptable (`parent.IsAttackInterruptable`))
  (return _interruptable))

(fn `UserConstructionScript`
  (`parent.UserConstructionScript`))

(fn `WasActorHitBefore`
  (params (TriggeringActor :type "Actor Object Reference") (ColliderComponent :type "PrimitiveComponent Object Reference"))
  (returns (ReturnValue :type Boolean))
  (bind _returnvalue (`MovesetComponent.WasActorHitBefore` (`self.Moveset`) TriggeringActor ColliderComponent))
  (return _returnvalue))