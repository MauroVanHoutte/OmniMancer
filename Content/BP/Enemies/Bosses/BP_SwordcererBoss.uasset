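; Swordcerer boss enemy that fights with four swords arranged around it, driven by a Moveset component.
; Move start and end events are matched by tag to spinning swords, push-out and sword charge handlers, which set state flags.
; Tick interpolates the sword colliders toward each attack's formation or back to default, blocking new attacks while rearranging.
; For the spin, the sword root detaches and follows the capsule's location, then reattaches afterward.
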(event `self.ReceiveBeginPlay`
  (`parent.ReceiveBeginPlay`)
  (`CollisionProfileMaterialChange.Initialize` (`self.CollisionProfileMaterialChange`) (`|MakeMap` (`self.SwordCollider`) (`self.Sword`) (`self.SwordCollider1`) (`self.Sword1`) (`self.SwordCollider2`) (`self.Sword2`) (`self.SwordCollider3`) (`self.Sword3`) :!type "PrimitiveComponent Object Reference" :!valuetype "MeshComponent Object Reference"))
  (bind _returnvalue (`KismetSystemLibrary.K2_SetTimerDelegate` (`|CreateDelegate` :!event `CustomEvent`) 3.0))
  (set `self.CooldownTimer` _returnvalue))

(event `self.ReceiveTick`
  (params (DeltaSeconds :type "Float (single-precision)"))
  (`parent.ReceiveTick` DeltaSeconds)
  (`self.TickSpinningSwordsAttack` DeltaSeconds)
  (`self.TickPushOutAttack` DeltaSeconds)
  (`self.TickSwordCharge` DeltaSeconds)
  (if (`self.bArrangingSwords`)
    (`|ExecutionSequence`
      (:`then_0`
        (bind _targetsreached (`self.ArrangeSwords` DeltaSeconds (`self.SwordDefaultTransforms`)))
        (if (and _targetsreached (== (`SceneComponent.RelativeRotation` (`self.SwordRoot`)) (struct) :`ErrorTolerance` 0.001)) :!label _label
          (set `self.bArrangingSwords` false)))
      (:`then_1`
        (`SceneComponent.K2_SetRelativeRotation` (`self.SwordRoot`) (`KismetMathLibrary.RInterpTo_Constant` (`SceneComponent.RelativeRotation` (`self.SwordRoot`)) (struct) DeltaSeconds (`self.SwordRearrangeRotationSpeed`)) false false))
      (:`then_2`
        (goto _label)))))

(event `self.Moveset.OnSubMoveCompletedDelegate`
  (params (MoveComponent :type "MovesetComponent Object Reference") (Move :type "BaseMove Object Reference"))
  (`self.AttackEnded` Move))

(event `self.Moveset.OnAttackCompletedDelegate`
  (params (MoveComponent :type "MovesetComponent Object Reference") (Move :type "BaseMove Object Reference"))
  (`self.AttackEnded` Move)
  (bind _returnvalue (`KismetSystemLibrary.K2_SetTimerDelegate` (delegate `CustomEvent`) 1.0))
  (set `self.CooldownTimer` _returnvalue))

(event `self.Moveset.OnAttackInterruptedDelegate`
  (params (MoveComponent :type "MovesetComponent Object Reference") (Move :type "BaseMove Object Reference"))
  (`self.AttackEnded` Move))

(event `CustomEvent`)

(event `self.Moveset.OnMoveExecutionStartedDelegate`
  (params (MoveComponent :type "MovesetComponent Object Reference") (Move :type "BaseMove Object Reference"))
  (`self.MoveExecutionStarted` Move))

(fn `ArrangeSwords`
  (params (DeltaTime :type "Float (double-precision)") (TargetTransforms :type "Array of Transform Structure"))
  (returns (TargetsReached :type Boolean))
  (bind _swordcollider (`self.SwordCollider`))
  (bind _swordcollider1 (`self.SwordCollider1`))
  (bind _swordcollider2 (`self.SwordCollider2`))
  (bind _swordcollider3 (`self.SwordCollider3`))
  (bind (_output_location _output_rotation) (`KismetMathLibrary.BreakTransform` (`|GetArrayItem` (`local.TargetTransforms`) 1)))
  (bind (_output_location_2 _output_rotation_2) (`KismetMathLibrary.BreakTransform` (`|GetArrayItem` (`local.TargetTransforms`) 2)))
  (bind (_output_location_3 _output_rotation_3) (`KismetMathLibrary.BreakTransform` (`|GetArrayItem` (`local.TargetTransforms`) 3)))
  (bind (_output_location_4 _output_rotation_4) (`KismetMathLibrary.BreakTransform` (`|GetArrayItem` (`local.TargetTransforms`))))
  (`|ExecutionSequence`
    (:`then_0`
      (`SceneComponent.K2_SetRelativeLocationAndRotation` _swordcollider (`KismetMathLibrary.VInterpTo_Constant` (`SceneComponent.RelativeLocation` _swordcollider) _output_location_4 (`local.DeltaTime`) (`self.SwordRearrangeSpeed`)) (`KismetMathLibrary.RInterpTo_Constant` (`SceneComponent.RelativeRotation` _swordcollider) _output_rotation_4 (`local.DeltaTime`) (`self.SwordRearrangeRotationSpeed`)) false false))
    (:`then_1`
      (`SceneComponent.K2_SetRelativeLocationAndRotation` _swordcollider1 (`KismetMathLibrary.VInterpTo_Constant` (`SceneComponent.RelativeLocation` _swordcollider1) _output_location (`local.DeltaTime`) (`self.SwordRearrangeSpeed`)) (`KismetMathLibrary.RInterpTo_Constant` (`SceneComponent.RelativeRotation` _swordcollider1) _output_rotation (`local.DeltaTime`) (`self.SwordRearrangeRotationSpeed`)) false false))
    (:`then_2`
      (`SceneComponent.K2_SetRelativeLocationAndRotation` _swordcollider2 (`KismetMathLibrary.VInterpTo_Constant` (`SceneComponent.RelativeLocation` _swordcollider2) _output_location_2 (`local.DeltaTime`) (`self.SwordRearrangeSpeed`)) (`KismetMathLibrary.RInterpTo_Constant` (`SceneComponent.RelativeRotation` _swordcollider2) _output_rotation_2 (`local.DeltaTime`) (`self.SwordRearrangeRotationSpeed`)) false false))
    (:`then_3`
      (`SceneComponent.K2_SetRelativeLocationAndRotation` _swordcollider3 (`KismetMathLibrary.VInterpTo_Constant` (`SceneComponent.RelativeLocation` _swordcollider3) _output_location_3 (`local.DeltaTime`) (`self.SwordRearrangeSpeed`)) (`KismetMathLibrary.RInterpTo_Constant` (`SceneComponent.RelativeRotation` _swordcollider3) _output_rotation_3 (`local.DeltaTime`) (`self.SwordRearrangeRotationSpeed`)) false false))
    (:`then_4`
      (return (and (== (`SceneComponent.GetRelativeTransform` (`self.SwordCollider`)) (`|GetArrayItem` (`local.TargetTransforms`))) (== (`SceneComponent.GetRelativeTransform` (`self.SwordCollider1`)) (`|GetArrayItem` (`local.TargetTransforms`) 1)) (== (`SceneComponent.GetRelativeTransform` (`self.SwordCollider2`)) (`|GetArrayItem` (`local.TargetTransforms`) 2)) (== (`SceneComponent.GetRelativeTransform` (`self.SwordCollider3`)) (`|GetArrayItem` (`local.TargetTransforms`) 3)))))))

(fn `Attack`
  (params (Target :type "Actor Object Reference"))
  (bind _returnvalue (`MovesetComponent.ExecuteAttack` (`self.Moveset`) Target))
  (if (not (`KismetSystemLibrary.IsValid` _returnvalue))
    (`self.AttackComplete`)))

(fn `AttackEnded`
  (params (Move :type "BaseMove Object Reference"))
  (bind _asattack_move (cast `AttackMove` Move))
  (bind _returnvalue (`AttackMove.GetAttackObject` _asattack_move))
  (`|ExecutionSequence`
    (:`then_0`
      (bind _returnvalue_2 (`BaseAttackObject.CompareTag` _returnvalue (`self.SpinningSwordsTag`)))
      (if _returnvalue_2
        (`self.HandleSpinningSwordsAttackEnded`)))
    (:`then_1`
      (bind _returnvalue_3 (`BaseAttackObject.CompareTag` _returnvalue (`self.PushOutTag`)))
      (if _returnvalue_3
        (`self.HandlePushOutCompleted`)))
    (:`then_2`
      (bind _returnvalue_4 (`BaseAttackObject.CompareTag` _returnvalue (`self.SwordChargeTag`)))
      (if _returnvalue_4
        (`self.HandleSwordChargeCompleted`)))))

(fn `CanAttack`
  (params (Target :type "Actor Object Reference"))
  (returns (CanAttack :type Boolean))
  (bind _canattack (`parent.CanAttack` Target))
  (return (and _canattack (not (`self.bArrangingSwords`)))))

(fn `HandlePushOutCompleted`
  (set `self.bArrangingSwords` true)
  (set `self.bSwordMovingToPushOut` false))

(fn `HandlePushOutStarted`
  (set `self.bSwordMovingToPushOut` true)
  (set `self.bArrangingSwords` false))

(fn `HandleSpinningSwordsAttackEnded`
  (set `self.bArrangingSwords` true)
  (set `self.bSpreadingSwords` false)
  (`SceneComponent.K2_AttachToComponent` (`self.SwordRoot`) (`self.CapsuleComponent`) "None" "SnapToTarget" "KeepRelative" "KeepRelative" false))

(fn `HandleSpinningSwordsAttackStarted`
  (set `self.bSpreadingSwords` true)
  (set `self.bArrangingSwords` false)
  (`SceneComponent.K2_DetachFromComponent` (`self.SwordRoot`) "KeepWorld" "KeepWorld" "KeepRelative" true)
  (set `self.bSwordSpinning` true))

(fn `HandleSwordChargeCompleted`
  (set `self.bArrangingSwords` true)
  (set `self.bSwordsMovingToSwordCharge` false))

(fn `HandleSwordChargeStarted`
  (set `self.bSwordsMovingToSwordCharge` true)
  (set `self.bArrangingSwords` false))

(fn `MoveExecutionStarted`
  (params (Move :type "BaseMove Object Reference"))
  (bind _asattack_move (cast `AttackMove` Move))
  (bind _returnvalue (`AttackMove.GetAttackObject` _asattack_move))
  (`|ExecutionSequence`
    (:`then_0`
      (bind _returnvalue_2 (`BaseAttackObject.CompareTag` _returnvalue (`self.SpinningSwordsTag`)))
      (if _returnvalue_2
        (`self.HandleSpinningSwordsAttackStarted`)))
    (:`then_1`
      (bind _returnvalue_3 (`BaseAttackObject.CompareTag` _returnvalue (`self.PushOutTag`)))
      (if _returnvalue_3
        (`self.HandlePushOutStarted`)))
    (:`then_2`
      (bind _returnvalue_4 (`BaseAttackObject.CompareTag` _returnvalue (`self.SwordChargeTag`)))
      (if _returnvalue_4
        (`self.HandleSwordChargeStarted`)))))

(fn `TickPushOutAttack`
  (params (DeltaTime :type "Float (double-precision)"))
  (`|ExecutionSequence`
    (:`then_0`
      (if (`self.bSwordMovingToPushOut`)
        (bind _targetsreached (`self.ArrangeSwords` (`local.DeltaTime`) (`self.SwordPushOutTranforms`)))
        (if _targetsreached
          (set `self.bSwordMovingToPushOut` false))))))

(fn `TickSpinningSwordsAttack`
  (params (DeltaTime :type "Float (double-precision)"))
  (`|ExecutionSequence`
    (:`then_0`
      (if (`self.bSpreadingSwords`)
        (bind _targetsreached (`self.ArrangeSwords` DeltaTime (`self. RotationAttackTransform`)))
        (if _targetsreached
          (set `self.bSpreadingSwords` false))))
    (:`then_1`
      (if (`self.bSwordSpinning`)
        (`SceneComponent.K2_SetWorldLocation` (`self.SwordRoot`) (`SceneComponent.K2_GetComponentLocation` (`self.CapsuleComponent`)) false false)))))

(fn `TickSwordCharge`
  (params (DeltaTime :type "Float (double-precision)"))
  (if (`self.bSwordsMovingToSwordCharge`)
    (bind _targetsreached (`self.ArrangeSwords` (`local.DeltaTime`) (`self.SwordChargeSwordTransforms`)))
    (if _targetsreached
      (set `self.bSwordsMovingToSwordCharge` false))))

(fn `UserConstructionScript`
  (`parent.UserConstructionScript`))