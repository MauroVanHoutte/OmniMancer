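; Projectile minion enemy Blueprint that keeps its AI controller focused on a target between attacks.
; BindComponents initializes target acquisition with the controller and affiliation, acquires the first target and sets focus through BP_BaseComponentController.
; It also binds base and decaying health to healthbars and shows the enemy widget.
; Whenever a Moveset attack completes or is interrupted, it reacquires a target and refocuses the controller.
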(event `self.ReceiveBeginPlay`
  (`parent.ReceiveBeginPlay`))

(event `self.Moveset.OnAttackCompletedDelegate`
  (params (MoveComponent :type "MovesetComponent Object Reference"))
  (`TargetAcquisitionComponent.AcquireTarget` (`self.TargetAcquisition`) :!label _label)
  (bind _asbp_base_component_controller (cast `/Game/BP/AI/BP_BaseComponentController` (`AIBlueprintHelperLibrary.GetAIController` self)))
  (`/Game/BP/AI/BP_BaseComponentController.SetFocusToTarget` _asbp_base_component_controller))

(event `self.Moveset.OnAttackInterruptedDelegate`
  (params (MoveComponent :type "MovesetComponent Object Reference"))
  (goto _label))

(fn `BindComponents`
  (bind _enemywidget (`self.EnemyWidget`))
  (`parent.BindComponents`)
  (`TargetAcquisitionComponent.Initialize` (`self.TargetAcquisition`) (`AIBlueprintHelperLibrary.GetAIController` self) (`self.AffiliationComponent`))
  (`TargetAcquisitionComponent.AcquireTarget` (`self.TargetAcquisition`))
  (bind _asbp_base_component_controller (cast `/Game/BP/AI/BP_BaseComponentController` (`AIBlueprintHelperLibrary.GetAIController` self)))
  (`/Game/BP/AI/BP_BaseComponentController.SetFocusToTarget` _asbp_base_component_controller)
  (`BaseHealthComponent.BindHealthbar` (`self.BaseHealthComponent`) null)
  (bind _asbp_enemy_widget (cast `/Game/UI/BP_EnemyWidget` (`WidgetComponent.GetUserWidgetObject` _enemywidget)))
  (`BaseHealthComponent.BindHealthbar` (`self.DecayingHealth`) (`/Game/UI/BP_EnemyWidget.BP_Healthbar` _asbp_enemy_widget))
  (`SceneComponent.SetVisibility` _enemywidget true false))

(fn `UserConstructionScript`
  (`parent.UserConstructionScript`))