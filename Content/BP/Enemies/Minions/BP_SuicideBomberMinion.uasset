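; Suicide bomber enemy minion Blueprint that adds target acquisition on top of its parent class.
; Component binding initializes TargetAcquisition with the AI controller and affiliation component, then acquires an initial target.
; It acquires a target again whenever a Moveset attack completes or is interrupted.
; No explosion or self-destruct logic appears in this Blueprint's graphs.
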(event `self.ReceiveBeginPlay`
  (`parent.ReceiveBeginPlay`))

(event `self.Moveset.OnAttackCompletedDelegate`
  (params (MoveComponent :type "MovesetComponent Object Reference"))
  (`TargetAcquisitionComponent.AcquireTarget` (`self.TargetAcquisition`) :!label _label))

(event `self.Moveset.OnAttackInterruptedDelegate`
  (params (MoveComponent :type "MovesetComponent Object Reference"))
  (goto _label))

(fn `BindComponents`
  (`parent.BindComponents`)
  (`TargetAcquisitionComponent.Initialize` (`self.TargetAcquisition`) (`AIBlueprintHelperLibrary.GetAIController` self) (`self.AffiliationComponent`))
  (`TargetAcquisitionComponent.AcquireTarget` (`self.TargetAcquisition`)))

(fn `UserConstructionScript`
  (`parent.UserConstructionScript`))