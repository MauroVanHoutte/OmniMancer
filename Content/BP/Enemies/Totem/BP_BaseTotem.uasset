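; Base totem enemy that automatically attacks the nearest pawn in its Range that has a different affiliation or none.
; Attacks chain through Moveset completion or failure, waiting for a Range overlap when no target exists.
; Moveset hits are forwarded as spell hits through a proxy bound to the instigator's trigger handling component.
; Components handle incoming hits and the healthbar, and fatal damage interrupts attacks before destroying the totem.
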(event `self.ReceiveBeginPlay`
  (`self.SetupHitHandling`)
  (`self.SetupHealthbar`)
  (`self.SetupProxyTriggerHandling`)
  (`self.Attack`))

(event `Attack`
  (bind (_target _targetfound) (`self.GetTarget`))
  (if _targetfound
    (bind _returnvalue (`MovesetComponent.ExecuteAttack` (`self.Moveset`) _target))
    (if (not _returnvalue)
      (`self.Attack`))
    (else
      (set `self.AwaitingTarget` true))))

(event `self.Range.OnComponentBeginOverlap`
  (params (OverlappedComponent :type "PrimitiveComponent Object Reference") (OtherActor :type "Actor Object Reference") (OtherComp :type "PrimitiveComponent Object Reference") (OtherBodyIndex :type Integer) (bFromSweep :type Boolean) (SweepResult :type "HitResult Structure (by ref)"))
  (if (`self.AwaitingTarget`)
    (set `self.AwaitingTarget` false)
    (`self.Attack`)))

(event `self.Moveset.OnAttackCompletedDelegate`
  (params (MoveComponent :type "MovesetComponent Object Reference"))
  (`self.Attack`))

(event `self.HealthManager.OnFatalDamageTakenDelegate`
  (params (DamagedComponent :type "BaseHealthComponent Object Reference") (Damage :type "Float (single-precision)") (OverkillDamage :type "Float (single-precision)") (DamageType :type "DamageType Object Reference") (InstigatedBy :type "Controller Object Reference") (DamageCauser :type "Actor Object Reference"))
  (`MovesetComponent.InterruptAttack` (`self.Moveset`))
  (`KismetSystemLibrary.Delay` 0.2)
  (`self.K2_DestroyActor`))

(event `HitTriggerInterface.OnTriggered`
  (params (TriggeringActor :type "Actor Object Reference") (ColliderComponent :type "PrimitiveComponent Object Reference"))
  (`MovesetComponent.OnHitTriggered` (`self.Moveset`) TriggeringActor ColliderComponent))

(event `self.Moveset.OnAttackHitDelegate`
  (params (MoveComponent :type "MovesetComponent Object Reference") (AttackActor :type "Actor Object Reference") (HitActor :type "Actor Object Reference"))
  (bind _asbase_spell (cast `BaseSpell` AttackActor)
    (:`then`
      _)
    (:`CastFailed`
      _))
  (`TriggerHandlingComponent.TriggerSpellHit` (`self.ProxyTriggerHandling`) _asbase_spell HitActor))

(fn `GetAffiliation`
  (returns (ReturnValue :type "AffiliationComponent Object Reference"))
  (return (`self.Affiliation`)))

(fn `GetTarget`
  (returns (Target :type "Actor Object Reference") (TargetFound :type Boolean))
  (locals (FilteredActors :type "Array of Actor Object Reference") (Closest :type "Float (double-precision)") (ClosestActor :type "Actor Object Reference"))
  (bind _closestactor (`local.ClosestActor`))
  (set `local.ClosestActor` null)
  (`KismetArrayLibrary.Array_Clear` (`local.FilteredActors`))
  (set `local.Closest` 1000000.0)
  (for _array_element (`PrimitiveComponent.GetOverlappingActors` (`self.Range`) "/Script/Engine.Pawn")
    (bind _returnvalue (`self.GetComponentByClass` _array_element "/Script/UnrealProject.AffiliationComponent"))
    (if (`KismetSystemLibrary.IsValid` _returnvalue)
      (if (`|EnumInequality` (`AffiliationComponent.GetAffiliation` (`self.Affiliation`)) (`AffiliationComponent.GetAffiliation` _returnvalue))
        (`KismetArrayLibrary.Array_Add` (`local.FilteredActors`) _array_element :!label _label))
      (else
        (goto _label))))
  (for _array_element_2 (`local.FilteredActors`)
    (bind _returnvalue_2 (`self.GetSquaredDistanceTo` _array_element_2 self))
    (if (< _returnvalue_2 (`local.Closest`))
      (set `local.Closest` _returnvalue_2)
      (set `local.ClosestActor` _array_element_2)))
  (return _closestactor (`KismetSystemLibrary.IsValid` _closestactor)))

(fn `SetupHealthbar`
  (bind _asbp_enemy_widget (cast `/Game/UI/BP_EnemyWidget` (`WidgetComponent.GetUserWidgetObject` (`self.Widget`))))
  (`BaseHealthComponent.BindHealthbar` (`self.DecayingHealth`) (`/Game/UI/BP_EnemyWidget.BP_Healthbar` _asbp_enemy_widget)))

(fn `SetupHitHandling`
  (`HitHandlingComponent.Initialize` (`self.HitHandling`) (`|MakeArray` (`self.Capsule`) :!type "ShapeComponent Object Reference") (`self.Affiliation`)))

(fn `SetupProxyTriggerHandling`
  (bind _returnvalue (`self.GetInstigator`))
  (bind _returnvalue_2 (`self.GetComponentByClass` _returnvalue "/Script/UnrealProject.TriggerHandlingComponent"))
  (`/Engine/EditorBlueprintResources/StandardMacros.IsValid` _returnvalue
    (:`Is Valid`
      (`/Engine/EditorBlueprintResources/StandardMacros.IsValid` _returnvalue_2
        (:`Is Valid`
          (`ProxyTriggerHandlingComponent.BindProxiedComponent` (`self.ProxyTriggerHandling`) _returnvalue_2))))))

(fn `UserConstructionScript`)

(fn `WasActorHitBefore`
  (params (TriggeringActor :type "Actor Object Reference") (ColliderComponent :type "PrimitiveComponent Object Reference"))
  (returns (ReturnValue :type Boolean))
  (bind _returnvalue (`MovesetComponent.WasActorHitBefore` (`self.Moveset`) TriggeringActor ColliderComponent))
  (return _returnvalue))