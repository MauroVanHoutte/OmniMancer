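; Spinner totem enemy, derived from a parent class, that extends its damage collider before starting its attack.
; On BeginPlay it clears the awaiting-target flag, stores the collider's Y scale as full size and shrinks it to near zero.
; Tick lerps the collider's Y scale back up over the grow duration, then stops growing and executes the attack through its Moveset.
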(event `self.ReceiveBeginPlay`
  (set `self.AwaitingTarget` false)
  (`parent.ReceiveBeginPlay`)
  (`self.StartGrowing`))

(event `self.ReceiveTick`
  (params (DeltaSeconds :type "Float (single-precision)"))
  (bind _damagecollider (`self.DamageCollider`))
  (bind (_relativescale3d_x _relativescale3d_y _relativescale3d_z) (`KismetMathLibrary.BreakVector` (`SceneComponent.RelativeScale3D` _damagecollider)))
  (`parent.ReceiveTick` DeltaSeconds)
  (if (`self.bGrowing`)
    (bind _output_get (set `self.GrowTimer` (+ DeltaSeconds (`self.GrowTimer`))))
    (`SceneComponent.SetRelativeScale3D` _damagecollider (`KismetMathLibrary.MakeVector` _relativescale3d_x (`KismetMathLibrary.FMin` (`KismetMathLibrary.Lerp` 0.0 (`self.Fullsize`) (/ _output_get (`self.GrowDuration`))) (`self.Fullsize`)) _relativescale3d_z))
    (if (> (`self.GrowTimer`) (`self.GrowDuration`))
      (set `self.bGrowing` false)
      (`self.Attack`))))

(event `self.ReceiveDestroyed`)

(fn `Attack`
  (`MovesetComponent.ExecuteAttack` (`self.Moveset`) null))

(fn `StartGrowing`
  (bind (_relativescale3d_x _relativescale3d_y _relativescale3d_z) (`KismetMathLibrary.BreakVector` (`SceneComponent.RelativeScale3D` (`self.DamageCollider`))))
  (set `self.Fullsize` _relativescale3d_y)
  (`SceneComponent.SetRelativeScale3D` (`self.DamageCollider`) (`KismetMathLibrary.MakeVector` _relativescale3d_x 0.001 _relativescale3d_z))
  (set `self.GrowTimer` 0.0)
  (set `self.bGrowing` true))

(fn `UserConstructionScript`
  (`parent.UserConstructionScript`))