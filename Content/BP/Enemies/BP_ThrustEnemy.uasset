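; Enemy that attacks by lunging at the player's position captured during charge-up, damaging wizard characters it passes through.
; ChargeAttack stores start and target locations and faces the target; Attack starts the leap and enables box overlaps.
; Tick moves it without sweep, using VInterpTo with accumulated time as a lerp over LeapDuration, then disables collision and signals completion.
; A HitActors list limits damage to once per wizard per leap.
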(event `self.ReceiveTick`
  (params (DeltaSeconds :type "Float (single-precision)"))
  (bind _leapduration (`self.LeapDuration`))
  (`parent.ReceiveTick` DeltaSeconds)
  (if (`self.Leaping`)
    (bind _output_get (set `self.LeapTime` (+ DeltaSeconds (`self.LeapTime`))))
    (`self.K2_SetActorLocation` (`KismetMathLibrary.VInterpTo` (`self.LeapStart`) (`self.Target`) _output_get (/ 1.0 _leapduration)) false true)
    (if (> _output_get _leapduration)
      (set `self.Leaping` false)
      (`PrimitiveComponent.SetCollisionProfileName` (`self.Box`) "NoCollision" true)
      (set `self.LeapTime` 0.0)
      (`KismetArrayLibrary.Array_Clear` (`self.HitActors`))
      (`self.AttackComplete`))))

(event `self.Box.OnComponentBeginOverlap`
  (params (OverlappedComponent :type "PrimitiveComponent Object Reference") (OtherActor :type "Actor Object Reference") (OtherComp :type "PrimitiveComponent Object Reference") (OtherBodyIndex :type Integer) (bFromSweep :type Boolean) (SweepResult :type "HitResult Structure (by ref)"))
  (bind _hitactors (`self.HitActors`))
  (bind _asbp_wizard_character (cast `/Game/BP/Wizards/BP_WizardCharacter` OtherActor))
  (if (not (`KismetArrayLibrary.Array_Contains` _hitactors _asbp_wizard_character))
    (`KismetArrayLibrary.Array_Add` _hitactors _asbp_wizard_character)
    (`self.TakeSpellDamageFloat` _asbp_wizard_character (`self.Damage`) self)))

(fn `Attack`
  (`parent.Attack`)
  (set `self.Leaping` true)
  (`PrimitiveComponent.SetCollisionProfileName` (`self.Box`) "OverlapAllDynamic" true))

(fn `ChargeAttack`
  (locals (Player :type Name :default "Player"))
  (bind _returnvalue (`self.GetController`))
  (`parent.ChargeAttack`)
  (bind _asaicontroller (cast `AIController` _returnvalue))
  (`AIController.K2_SetFocus` _asaicontroller null)
  (bind _asactor (cast `Actor` (`BlackboardComponent.GetValueAsObject` (`AIBlueprintHelperLibrary.GetBlackboard` _returnvalue) (`local.Player`))))
  (bind _output_get (set `self.Target` (`self.K2_GetActorLocation` _asactor)))
  (bind _output_get_2 (set `self.LeapStart` (`self.K2_GetActorLocation`)))
  (`self.K2_SetActorRotation` (`KismetMathLibrary.Conv_VectorToRotator` (- _output_get _output_get_2))))

(fn `UserConstructionScript`
  (`parent.UserConstructionScript`))