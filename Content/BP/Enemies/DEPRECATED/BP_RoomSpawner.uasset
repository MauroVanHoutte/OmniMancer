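; Wave-based room spawner, in a DEPRECATED folder, that locks the exit portal until all enemy waves have spawned.
; A wizard leaving the landing zone sets pack sizes from its combined element level, locks the portal and starts the first wave.
; Tick spawns later waves via a Delay, then unlocks the portal.
; Each wave fills tagged melee, ranged and special boxes with weighted-random enemies at random points.
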(event `self.ReceiveBeginPlay`
  (add `/Game/BP/BP_Portal.ResetSpawner` (`self.ExitPortal`) (`|CreateDelegate` :!event `Reset`)))

(event `self.ReceiveTick`
  (params (DeltaSeconds :type "Float (single-precision)"))
  (bind _timebetweenwaves (`self.TimeBetweenWaves`))
  (if (>= (`self.CurrentWave`) (`self.TotalWaves`))
    (set `self.Active` false)
    (`self.Unlock`)
    (elif (and (> _timebetweenwaves 0.0) (`self.Active`))
      (`KismetSystemLibrary.Delay` _timebetweenwaves)
      (`self.SpawnWave`))))

(event `self.LandingZone.OnComponentEndOverlap`
  (params (OverlappedComponent :type "PrimitiveComponent Object Reference") (OtherActor :type "Actor Object Reference") (OtherComp :type "PrimitiveComponent Object Reference") (OtherBodyIndex :type Integer))
  (bind _asbp_wizard_character (cast `/Game/BP/Wizards/BP_WizardCharacter` OtherActor))
  (set `self.WizardLevel` (`WizardCharacter.GetCombinedElementLevel` _asbp_wizard_character))
  (`self.SetDifficulty`)
  (set `self.Active` true)
  (`/Game/BP/BP_Portal.Lock` (`self.ExitPortal`))
  (if (< (`self.CurrentWave`) 1)
    (`self.SpawnWave`)))

(event `Unlock`
  (`/Game/BP/BP_Portal.Unlock` (`self.ExitPortal`)))

(fn `Get Random Spawnable Enemy Type`
  (params (EnemyPool :type "Map of /Game/BP/Enemies/BP_BaseEnemy Class Reference to Float (double-precision)"))
  (returns (EnemyType :type "/Game/BP/Enemies/BP_BaseEnemy Class Reference"))
  (locals (TotalWeight :type "Float (double-precision)") (RandomResult :type "Float (double-precision)"))
  (bind _randomresult (`local.RandomResult`))
  (set `local.TotalWeight` 0.0)
  (bind _values (`BlueprintMapLibrary.Map_Values` EnemyPool))
  (for _array_element _values
    (set `local.TotalWeight` (+ _array_element (`local.TotalWeight`))))
  (set `local.RandomResult` (`KismetMathLibrary.RandomFloatInRange` 0.0 (`local.TotalWeight`)))
  (for (_array_element_2 _array_index) _values
    (if (< _randomresult _array_element_2)
      (bind _keys (`BlueprintMapLibrary.Map_Keys` EnemyPool))
      (return (`|GetArrayItem` _keys _array_index))
      (else
        (set `local.RandomResult` (- _randomresult _array_element_2))))))

(fn `GetSpawnLocation`
  (params (box :type "BoxComponent Object Reference"))
  (returns (Location :type "Vector Structure"))
  (if (`KismetSystemLibrary.IsValid` box)
    (return (`KismetMathLibrary.RandomPointInBoundingBox` (`SceneComponent.K2_GetComponentLocation` box) (`BoxComponent.GetScaledBoxExtent` box)))))

(fn `Reset`
  (set `self.CurrentWave` 0))

(fn `SetDifficulty`
  (set `self.MinPackSize` (+ (/ (`self.WizardLevel`) 4) 1))
  (set `self.MaxPackSize` (+ (/ (`self.WizardLevel`) 2) 1)))

(fn `SpawnEnemies`
  (params (ZoneTag :type Name) (EnemyPool :type "Map of /Game/BP/Enemies/BP_BaseEnemy Class Reference to Float (double-precision)"))
  (bind _returnvalue (`self.GetComponentsByTag` "/Script/Engine.BoxComponent" ZoneTag))
  (bind _minpacksize (`self.MinPackSize`))
  (bind _returnvalue_2 (`KismetArrayLibrary.Array_Length` _returnvalue))
  (if (> _returnvalue_2 0)
    (for _index (range _returnvalue_2)
      (for _ (range _minpacksize (+ (`KismetMathLibrary.RandomIntegerInRange` _minpacksize (`self.MaxPackSize`)) 1))
        (bind _location (`self.GetSpawnLocation` (`|GetArrayItem` _returnvalue _index)))
        (bind _enemytype (`self.Get Random Spawnable Enemy Type` EnemyPool))
        (`|SpawnActorFromClass` _enemytype (`KismetMathLibrary.MakeTransform` _location (`KismetMathLibrary.MakeRotator` 0.0 0.0 (`KismetMathLibrary.RandomFloat`))) "AdjustIfPossibleButAlwaysSpawn" "SelectDefaultAtRuntime" null null)))))

(fn `SpawnWave`
  (`/Engine/EditorBlueprintResources/StandardMacros.IncrementInt` (`self.CurrentWave`)
    (:`  `
      (`|ExecutionSequence`
        (:`then_0`
          (`self.SpawnEnemies` "MeleeSpawnZone" (`self.EnemyTypesMelee`)))
        (:`then_1`
          (`self.SpawnEnemies` "RangedSpawnZone" (`self.EnemyTypesRanged`)))
        (:`then_2`
          (`self.SpawnEnemies` "SpecialSpawnZone" (`self.EnemyTypesSpecial`)))))))

(fn `UserConstructionScript`)