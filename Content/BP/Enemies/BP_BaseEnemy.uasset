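; Base enemy Blueprint that wires together health, stats, hit handling, status effects and a Moveset for attacks.
; BeginPlay initializes the components and binds the enemy widget's healthbar and status bar, which is made visible on damage.
; Attack, interrupt and hit queries delegate to the Moveset, while charge, post-attack and initiation functions are stubs.
; On fatal damage it launches BP_Coin experience orbs in random upward directions, then destroys itself.
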(event `self.ReceiveBeginPlay`
  (`HitHandlingComponent.Initialize` (`self.HitHandlingComponent`) (`|MakeArray` (`self.CapsuleComponent`) :!type "ShapeComponent Object Reference") (`self.AffiliationComponent`))
  (`StatComponent.Initialize` (`self.StatsComponent`) (`self.CharacterMovement`))
  (`ForceApplicationComponent.Initialize` (`self.ForceApplicationComponent`) (`self.CharacterMovement`))
  (bind _asbp_enemy_widget (cast `/Game/UI/BP_EnemyWidget` (`WidgetComponent.GetUserWidgetObject` (`self.EnemyWidget`))))
  (`StatusEffectHandlingComponent.BindStatusEffectsBar` (`self.StatusEffectHandlingComponent`) (`/Game/UI/BP_EnemyWidget.BP_ActiveStatusEffectsBar` _asbp_enemy_widget))
  (`BaseHealthComponent.BindHealthbar` (`self.BaseHealthComponent`) (`/Game/UI/BP_EnemyWidget.BP_Healthbar` _asbp_enemy_widget)))

(event `self.ReceiveTick`
  (params (DeltaSeconds :type "Float (single-precision)")))

(event `self.HealthManager.OnFatalDamageTakenDelegate`
  (params (DamagedComponent :type "BaseHealthComponent Object Reference") (Damage :type "Float (single-precision)") (OverkillDamage :type "Float (single-precision)") (DamageType :type "DamageType Object Reference") (InstigatedBy :type "Controller Object Reference") (DamageCauser :type "Actor Object Reference"))
  (`self.SpawnExperience`)
  (`KismetSystemLibrary.Delay` 0.2)
  (`self.K2_DestroyActor`))

(event `self.HealthManager.OnDamageTakenDelegate`
  (params (DamagedComponent :type "BaseHealthComponent Object Reference") (Damage :type "Float (single-precision)") (DamageType :type "DamageType Object Reference") (InstigatedBy :type "Controller Object Reference") (DamageCauser :type "Actor Object Reference"))
  (`SceneComponent.SetVisibility` (`self.EnemyWidget`) true false))

(event `self.Moveset.OnAttackCompletedDelegate`
  (params (MoveComponent :type "MovesetComponent Object Reference"))
  (`self.AttackComplete`))

(event `HitTriggerInterface.OnTriggered`
  (params (TriggeringActor :type "Actor Object Reference") (ColliderComponent :type "PrimitiveComponent Object Reference"))
  (`MovesetComponent.OnHitTriggered` (`self.Moveset`) TriggeringActor ColliderComponent))

(fn `Attack`
  (params (Target :type "Actor Object Reference"))
  (bind _returnvalue (`MovesetComponent.ExecuteAttack` (`self.Moveset`) Target))
  (if (not _returnvalue)
    (`self.AttackComplete`)))

(fn `CanAttack`
  (params (Target :type "Actor Object Reference"))
  (returns (CanAttack :type Boolean))
  (bind _returnvalue (`MovesetComponent.CanExecuteAttack` (`self.Moveset`) Target))
  (return _returnvalue))

(fn `ChargeAttack`)

(fn `GetAffiliation`
  (returns (ReturnValue :type "AffiliationComponent Object Reference"))
  (return (`self.AffiliationComponent`)))

(fn `InterruptAttack`
  (`MovesetComponent.InterruptAttack` (`self.Moveset`)))

(fn `IsAttackInterruptable`
  (returns (Interruptable :type Boolean))
  (bind _returnvalue (`MovesetComponent.CanBeInterrupted` (`self.Moveset`)))
  (return _returnvalue))

(fn `PostAttack`)

(fn `SpawnExperience`
  (locals (Angle :type "Float (double-precision)" :default 0.0))
  (for _ (range 1 (+ (`self.ExperienceOrbs`) 1))
    (bind _returnvalue (`|SpawnActorFromClass` "/Game/BP/BP_Coin.BP_Coin_C" (`KismetMathLibrary.MakeTransform` (`self.K2_GetActorLocation`)) "AdjustIfPossibleButAlwaysSpawn" "MultiplyWithRoot" null null))
    (bind _output_get (set `local.Angle` (`KismetMathLibrary.RandomFloatInRange` 0.0 (`KismetMathLibrary.MultiplyByPi` 2.0))))
    (`Coin.LaunchInDirection` _returnvalue (`KismetMathLibrary.Normal` (`KismetMathLibrary.MakeVector` (`KismetMathLibrary.Sin` _output_get) (`KismetMathLibrary.Cos` _output_get) 1.0)) 300.0)))

(fn `TryInitiateAttack`
  (returns (Succeeded :type Boolean))
  (return false))

(fn `UserConstructionScript`)

(fn `WasActorHitBefore`
  (params (TriggeringActor :type "Actor Object Reference") (ColliderComponent :type "PrimitiveComponent Object Reference"))
  (returns (ReturnValue :type Boolean))
  (bind _returnvalue (`MovesetComponent.WasActorHitBefore` (`self.Moveset`) TriggeringActor ColliderComponent))
  (return _returnvalue))