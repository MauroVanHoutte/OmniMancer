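; Enemy Blueprint for a mortar attacker that delegates its attack behaviour to a MortarAttack component.
; It overrides the parent's CanAttack, Attack, InterruptAttack and IsAttackInterruptable to forward to that component's requirement, initiate and interrupt functions.
; The component's attack-completed delegate calls AttackComplete on the enemy.
; CanAttack returns only the component's requirement check, ignoring the parent's result.
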(event `self.ReceiveBeginPlay`
  (`parent.ReceiveBeginPlay`))

(event `self.MortarAttack.AttackCompletedDelegate`
  (params (AttackComponent :type "BaseAttackComponent Object Reference"))
  (`self.AttackComplete`))

(fn `Attack`
  (`parent.Attack`)
  (`BaseAttackComponent.InitiateAttack` (`self.MortarAttack`)))

(fn `CanAttack`
  (returns (CanAttack :type Boolean))
  (`parent.CanAttack`)
  (bind _returnvalue (`BaseAttackComponent.AreAttackRequirementsMet` (`self.MortarAttack`)))
  (return _returnvalue))

(fn `InterruptAttack`
  (`parent.InterruptAttack`)
  (`BaseAttackComponent.TryInterruptAttack` (`self.MortarAttack`)))

(fn `IsAttackInterruptable`
  (returns (Interruptable :type Boolean))
  (bind _returnvalue (`BaseAttackComponent.IsAttackInterruptable` (`self.MortarAttack`)))
  (return _returnvalue))

(fn `UserConstructionScript`
  (`parent.UserConstructionScript`))