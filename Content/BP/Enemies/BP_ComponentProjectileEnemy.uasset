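; BP_ComponentProjectileEnemy is an enemy Blueprint that delegates its attack to a ProjectileAttack component.
; CanAttack calls the parent, then returns only the component's requirements check, and Attack calls the parent before initiating the component's attack.
; The component's completion delegate triggers CallAttackComplete, while BeginPlay and construction just call the parent, and Tick is disabled.
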(event `self.ReceiveBeginPlay`
  (`parent.ReceiveBeginPlay`))

(event `self.ProjectileAttack.AttackCompletedDelegate`
  (params (AttackComponent :type "BaseAttackComponent Object Reference"))
  (`self.AttackComplete`))

(fn `Attack`
  (`parent.Attack`)
  (`BaseAttackComponent.InitiateAttack` (`self.ProjectileAttack`)))

(fn `CanAttack`
  (returns (CanAttack :type Boolean))
  (`parent.CanAttack`)
  (bind _returnvalue (`BaseAttackComponent.AreAttackRequirementsMet` (`self.ProjectileAttack`)))
  (return _returnvalue))

(fn `UserConstructionScript`
  (`parent.UserConstructionScript`))