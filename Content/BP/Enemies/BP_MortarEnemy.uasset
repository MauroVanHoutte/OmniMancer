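; Mortar enemy Blueprint that lobs a BP_MortarProjectile at the first player pawn's current position.
; Attack spawns the projectile at the enemy, estimates flight time from InitialSpeed and Gravity, and divides player distance by it for horizontal velocity.
; It pairs that with a fixed upward speed, sets InitialSpeed to the resulting magnitude, then calls CallAttackComplete if the movement component is valid.
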(fn `Attack`
  (locals (Gravity :type "Float (double-precision)" :default 980.0))
  (bind _returnvalue (`self.K2_GetActorLocation`))
  (bind _returnvalue_2 (`self.K2_GetActorLocation` (`GameplayStatics.GetPlayerPawn` 0)))
  (bind _returnvalue_3 (`|SpawnActorFromClass` "/Game/BP/Enemies/BP_MortarProjectile.BP_MortarProjectile_C" (`KismetMathLibrary.MakeTransform` _returnvalue) "Undefined" "OverrideRootScale" self self))
  (bind _returnvalue_4 (`MortarProjectile.GetProjectileMovementComp` _returnvalue_3))
  (`/Engine/EditorBlueprintResources/StandardMacros.IsValid` _returnvalue_4
    (:`Is Valid`
      (bind (_returnvalue_x _returnvalue_y) (`KismetMathLibrary.BreakVector` (* (`KismetMathLibrary.Normal` (- _returnvalue_2 _returnvalue)) (/ (`KismetMathLibrary.Vector_Distance` _returnvalue _returnvalue_2) (/ (* (`ProjectileMovementComponent.InitialSpeed` _returnvalue_4) 2.0) (`local.Gravity`))))))
      (bind _returnvalue_5 (`KismetMathLibrary.MakeVector` _returnvalue_x _returnvalue_y 1000.0))
      (set `MovementComponent.Velocity` _returnvalue_5 _returnvalue_4)
      (set `ProjectileMovementComponent.InitialSpeed` (`KismetMathLibrary.VSize` _returnvalue_5) _returnvalue_4)
      (`self.AttackComplete`))))

(fn `UserConstructionScript`
  (`parent.UserConstructionScript`))