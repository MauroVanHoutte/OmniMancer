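; BP_RoomSpawner runs a room encounter, spawning enemy packs and controlling the exit portal.
; The wizard leaving LandingZone sets the spawn rate and locks the portal, which the Unlock event reopens.
; Tick uses a Delay to pace packs of random size at reachable points around a location in MeleeSpawnZone-tagged boxes.
; Each enemy class comes from a weighted random pick over the EnemyTypesMelee map.
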(event `self.ReceiveBeginPlay`
  (`self.GetSpawnLocation` "gjklsdjkl"))

(event `self.ReceiveTick`
  (params (DeltaSeconds :type "Float (single-precision)"))
  (bind _spawnrate (`self.SpawnRate`))
  (if (not (<= _spawnrate 0.0))
    (`KismetSystemLibrary.Delay` (/ 1.0 _spawnrate))
    (bind _location (`self.GetSpawnLocation` "MeleeSpawnZone"))
    (set `self.Random Location` _location)
    (for _ (range 1 (+ (`KismetMathLibrary.RandomIntegerInRange` (`self.MinPackSize`) (`self.MaxPackSize`)) 1))
      (bind _enemytype (`self.GetRandomSpawnableEnemyType`))
      (`|SpawnActorFromClass` _enemytype (`KismetMathLibrary.MakeTransform` (`NavigationSystemV1.K2_GetRandomReachablePointInRadius` (`self.Random Location`) (`self.PackRadius`) null null) (`KismetMathLibrary.MakeRotator` 0.0 0.0 (`KismetMathLibrary.RandomFloat`))) "Undefined" "OverrideRootScale" null null))))

(event `self.LandingZone.OnComponentEndOverlap`
  (params (OverlappedComponent :type "PrimitiveComponent Object Reference") (OtherActor :type "Actor Object Reference") (OtherComp :type "PrimitiveComponent Object Reference") (OtherBodyIndex :type Integer))
  (cast `/Game/BP/BP_WizardCharacter` OtherActor)
  (set `self.SpawnRate` 0.15)
  (`/Game/BP/BP_Portal.Lock` (`self.ExitPortal`)))

(event `Unlock`
  (`/Game/BP/BP_Portal.Unlock` (`self.ExitPortal`)))

(fn `GetRandomSpawnableEnemyType`
  (returns (EnemyType :type "/Game/BP/Enemies/BP_BaseEnemy Class Reference"))
  (locals (TotalWeight :type "Float (double-precision)") (RandomResult :type "Float (double-precision)"))
  (bind _randomresult (`local.RandomResult`))
  (set `local.TotalWeight` 0.0)
  (bind _values (`BlueprintMapLibrary.Map_Values` (`self.EnemyTypesMelee`)))
  (for _array_element _values
    (set `local.TotalWeight` (+ _array_element (`local.TotalWeight`))))
  (set `local.RandomResult` (`KismetMathLibrary.RandomFloatInRange` 0.0 (`local.TotalWeight`)))
  (for (_array_element_2 _array_index) _values
    (if (< _randomresult _array_element_2)
      (bind _keys (`BlueprintMapLibrary.Map_Keys` (`self.EnemyTypesMelee`)))
      (return (`|GetArrayItem` _keys _array_index))
      (else
        (set `local.RandomResult` (- _randomresult _array_element_2)))))
  (return null))

(fn `GetSpawnLocation`
  (params (AreaTag :type Name))
  (returns (Location :type "Vector Structure"))
  (bind _returnvalue (`self.GetComponentsByTag` "/Script/Engine.BoxComponent" AreaTag))
  (bind _returnvalue_2 (`KismetArrayLibrary.Array_Length` _returnvalue))
  (bind _output (`|GetArrayItem` _returnvalue (`KismetMathLibrary.RandomInteger` _returnvalue_2)))
  (if (> _returnvalue_2 0)
    (return (`KismetMathLibrary.RandomPointInBoundingBox` (`SceneComponent.K2_GetComponentLocation` _output) (`BoxComponent.GetScaledBoxExtent` _output)))
    (else
      (`KismetSystemLibrary.PrintString` (`KismetStringLibrary.Concat_StrStr` (`KismetStringLibrary.Concat_StrStr` (`KismetStringLibrary.Concat_StrStr` (`KismetSystemLibrary.GetObjectName` self) " doesnt have components with ") (`KismetStringLibrary.Conv_NameToString` AreaTag)) " tag") true true (struct :`G` 0.66 :`B` 1.0 :`A` 1.0) 10.0)
      (return (0.0 0.0 0.0)))))

(fn `Set Enemy Type Spawnable`
  (params (EnemyType :type "/Game/BP/Enemies/BP_BaseEnemy Class Reference") (SpawnWeight :type "Float (double-precision)"))
  (`BlueprintMapLibrary.Map_Add` (`self.EnemyTypesMelee`) EnemyType SpawnWeight))

(fn `UserConstructionScript`)