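; Suicide bomber enemy built on components, which deals damage through an area attack and destroys itself when that attack completes.
; The parent's attack, readiness and interruption functions are overridden to delegate to the AreaAttack component.
; The OnTriggered event applies Damage to the triggering actor, crediting the instigator controller.
; It also exposes its AffiliationComponent and a lookup of HitActors, which nothing in these graphs fills.
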(event `self.ReceiveTick`
  (params (DeltaSeconds :type "Float (single-precision)"))
  (`parent.ReceiveTick` DeltaSeconds))

(event `HitTriggerInterface.OnTriggered`
  (params (TriggeringActor :type "Actor Object Reference"))
  (`GameplayStatics.ApplyDamage` TriggeringActor (`self.Damage`) (`self.GetInstigatorController` self) self))

(event `self.AreaAttack.AttackCompletedDelegate`
  (params (AttackComponent :type "BaseAttackComponent Object Reference"))
  (`self.K2_DestroyActor`))

(fn `Attack`
  (`parent.Attack`)
  (`BaseAttackComponent.InitiateAttack` (`self.AreaAttack`)))

(fn `CanAttack`
  (returns (CanAttack :type Boolean))
  (`parent.CanAttack`)
  (bind _returnvalue (`BaseAttackComponent.AreAttackRequirementsMet` (`self.AreaAttack`)))
  (return _returnvalue))

(fn `GetAffiliation`
  (returns (ReturnValue :type "AffiliationComponent Object Reference"))
  (return (`self.AffiliationComponent`)))

(fn `InterruptAttack`
  (`parent.InterruptAttack`)
  (`BaseAttackComponent.TryInterruptAttack` (`self.AreaAttack`)))

(fn `IsAttackInterruptable`
  (returns (Interruptable :type Boolean))
  (bind _returnvalue (`BaseAttackComponent.IsAttackInterruptable` (`self.AreaAttack`)))
  (return _returnvalue))

(fn `UserConstructionScript`
  (`parent.UserConstructionScript`))

(fn `WasActorHitBefore`
  (params (TriggeringActor :type "Actor Object Reference"))
  (returns (ReturnValue :type Boolean))
  (return (`KismetArrayLibrary.Array_Contains` (`self.HitActors`) TriggeringActor)))