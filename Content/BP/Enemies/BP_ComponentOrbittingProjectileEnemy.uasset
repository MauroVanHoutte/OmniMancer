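; Orbiting projectile enemy that attacks in bursts, delegating each shot to its ProjectileAttack component.
; Attack resets the burst counter, and each completion callback from the component chains the next attack until AttacksPerBurst is reached.
; A cooldown timer then runs, with BurstCompleted signaling that the attack is complete.
; Readiness and interruptibility checks defer to the component, and interrupting also clears the timer.
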(event `self.ReceiveBeginPlay`
  (`parent.ReceiveBeginPlay`))

(event `self.ProjectileAttack.AttackCompletedDelegate`
  (params (AttackComponent :type "BaseAttackComponent Object Reference"))
  (bind _result (`/Engine/EditorBlueprintResources/StandardMacros.IncrementInt` (`self.CurrentAttack`))
    (:`  `
      (if (>= _result (`self.AttacksPerBurst`))
        (bind _returnvalue (`KismetSystemLibrary.K2_SetTimerDelegate` (`|CreateDelegate` :!event `BurstCompleted`) (`self.CooldownTime`)))
        (set `self.TimerHandle` _returnvalue)
        (else
          (`BaseAttackComponent.InitiateAttack` (`self.ProjectileAttack`)))))))

(event `BurstCompleted`
  (`/Game/BP/Enemies/BP_BaseEnemy.AttackComplete`))

(fn `Attack`
  (set `self.CurrentAttack` 0)
  (`BaseAttackComponent.InitiateAttack` (`self.ProjectileAttack`)))

(fn `CanAttack`
  (returns (CanAttack :type Boolean))
  (bind _returnvalue (`BaseAttackComponent.AreAttackRequirementsMet` (`self.ProjectileAttack`)))
  (return _returnvalue))

(fn `InterruptAttack`
  (`KismetSystemLibrary.K2_ClearAndInvalidateTimerHandle` (`self.TimerHandle`))
  (`BaseAttackComponent.TryInterruptAttack` (`self.ProjectileAttack`)))

(fn `IsAttackInterruptable`
  (returns (Interruptable :type Boolean))
  (bind _returnvalue (`BaseAttackComponent.IsAttackInterruptable` (`self.ProjectileAttack`)))
  (return _returnvalue))

(fn `UserConstructionScript`
  (`parent.UserConstructionScript`))