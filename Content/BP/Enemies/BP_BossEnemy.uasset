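; Boss enemy Blueprint that extends a parent enemy class with moveset-driven attacks gated by a cooldown.
; Attack hands the target to Moveset, then starts the cooldown timer on success or signals attack completion on failure.
; CanAttack requires both the parent check and an inactive cooldown timer, so the timer handle itself serves as the cooldown state.
; Interrupt logic simply defers to the parent.
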(event `AttackTimerCompleted`)

(fn `Attack`
  (params (Target :type "Actor Object Reference"))
  (bind _returnvalue (`MovesetComponent.ExecuteAttack` (`self.Moveset`) Target))
  (if _returnvalue
    (bind _returnvalue_2 (`KismetSystemLibrary.K2_SetTimerDelegate` (`|CreateDelegate` :!event `AttackTimerCompleted`) (`self.AttackCooldown`)))
    (set `self.AttackTimer` _returnvalue_2)
    (else
      (`self.AttackComplete`))))

(fn `CanAttack`
  (params (Target :type "Actor Object Reference"))
  (returns (CanAttack :type Boolean))
  (bind _canattack (`parent.CanAttack` Target))
  (return (and _canattack (not (`KismetSystemLibrary.K2_IsTimerActiveHandle` (`self.AttackTimer`))))))

(fn `InterruptAttack`
  (`parent.InterruptAttack`))

(fn `IsAttackInterruptable`
  (returns (Interruptable :type Boolean))
  (bind _interruptable (`parent.IsAttackInterruptable`))
  (return _interruptable))

(fn `UserConstructionScript`
  (`parent.UserConstructionScript`))