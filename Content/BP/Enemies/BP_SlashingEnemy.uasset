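; BP_SlashingEnemy is a sword-wielding enemy whose attack hits and completion are handled through its Moveset component.
; Trigger events pass the touched actor and collider to the Moveset, which also answers whether that actor was hit before.
; When the Moveset reports an attack completed, SwordRoot's relative rotation resets to zero.
; GetAffiliation exposes the AffiliationComponent.
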(event `self.Moveset.OnAttackCompletedDelegate`
  (params (MoveComponent :type "MovesetComponent Object Reference") (Move :type "BaseMove Object Reference"))
  (`SceneComponent.K2_SetRelativeRotation` :`self` (`self.SwordRoot`)))

(event `HitTriggerInterface.OnTriggered`
  (params (TriggeringActor :type "Actor Object Reference") (ColliderComponent :type "PrimitiveComponent Object Reference"))
  (`MovesetComponent.OnHitTriggered` (`self.Moveset`) TriggeringActor ColliderComponent))

(fn `GetAffiliation`
  (returns (ReturnValue :type "AffiliationComponent Object Reference"))
  (return (`self.AffiliationComponent`)))

(fn `UserConstructionScript`
  (`parent.UserConstructionScript`))

(fn `WasActorHitBefore`
  (params (TriggeringActor :type "Actor Object Reference") (ColliderComponent :type "PrimitiveComponent Object Reference"))
  (returns (ReturnValue :type Boolean))
  (bind _returnvalue (`MovesetComponent.WasActorHitBefore` (`self.Moveset`) TriggeringActor ColliderComponent))
  (return _returnvalue))