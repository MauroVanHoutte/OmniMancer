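; BP_WizardCharacter is the wizard character Blueprint, with a health bar widget and hooks for element and death events.
; Every Tick it casts the Healthbar component's widget to Healthbar and sets its percentage to current health divided by starting health.
; OnAddElement and OnDeath simply forward to CallElementAdded and CallDeath, whose logic is not defined in this graph.
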(event `self.ReceiveTick`
  (params (DeltaSeconds :type "Float (single-precision)"))
  (bind _ashealthbar (cast `/Game/UI/Healthbar` (`WidgetComponent.GetWidget` (`self.Healthbar`))))
  (bind _returnvalue (`self.GetHealth`))
  (bind _returnvalue_2 (`self.GetStartHealth`))
  (`/Game/UI/Healthbar.SetPercentage` _ashealthbar (/ _returnvalue _returnvalue_2)))

(event `self.OnAddElement`
  (`self.ElementAdded`))

(event `self.OnDeath`
  (`self.Death`))

(fn `UserConstructionScript`)