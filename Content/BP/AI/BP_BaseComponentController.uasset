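; BP_BaseComponentController is an AI controller that initializes BP_BaseEnemy pawns and manages their Blackboard target.
; Startup waits for both BeginPlay and Possess, in either order, then writes the player pawn to the Blackboard and calls the enemy's OnControllerBeginPlay.
; SetNewTarget writes the Blackboard target key, and SetFocusToTarget reads it back to set the AI's focus on that actor.
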(event `self.ReceiveBeginPlay`
  (bind _output_get (set `self.HasBegunPlay` true))
  (if (and _output_get (stale `self.ReceivePossess` _output_get)) :!label _label
    (`BlackboardComponent.SetValueAsObject` (`AIBlueprintHelperLibrary.GetBlackboard` null) (`self.Key Name`) (`GameplayStatics.GetPlayerPawn` 0))
    (bind _asbp_base_enemy (cast `/Game/BP/Enemies/BP_BaseEnemy` (`self.K2_GetPawn`)))
    (`/Game/BP/Enemies/BP_BaseEnemy.OnControllerBeginPlay` _asbp_base_enemy)))

(event `self.ReceivePossess`
  (params (PossessedPawn :type "Pawn Object Reference"))
  (bind _output_get (set `self.HasPossessed` true))
  (goto _label))

(fn `SetFocusToTarget`
  (locals (TargetKey :type Name :default "Target"))
  (bind _asactor (cast `Actor` (`BlackboardComponent.GetValueAsObject` (`AIBlueprintHelperLibrary.GetBlackboard` null) (`local.TargetKey`))))
  (`self.K2_SetFocus` _asactor))

(fn `SetNewTarget`
  (params (NewTarget :type "Actor Object Reference"))
  (locals (TargetKey :type Name :default "Target"))
  (`BlackboardComponent.SetValueAsObject` (`AIBlueprintHelperLibrary.GetBlackboard` null) (`local.TargetKey`) NewTarget))

(fn `UserConstructionScript`)