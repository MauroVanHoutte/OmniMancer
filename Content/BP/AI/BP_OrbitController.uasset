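; AI controller that runs the BP_OrbitBehaviour behavior tree and drives the orbit direction stored in its Blackboard.
; Direction starts positive on BeginPlay.
; Each tick, it focuses on the Blackboard's Player actor and counts down a timer, skipping both if no actor is set.
; When the timer expires, it flips the sign of OrbitDirection and picks a new short random interval, so direction changes irregularly.
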(event `self.ReceiveBeginPlay`
  (`parent.ReceiveBeginPlay`)
  (`self.RunBehaviorTree` "/Game/BP/AI/BP_OrbitBehaviour.BP_OrbitBehaviour")
  (`BlackboardComponent.SetValueAsFloat` (`self.Blackboard`) (`self.OrbitDirection`) 1.0))

(event `self.ReceiveTick`
  (params (DeltaSeconds :type "Float (single-precision)"))
  (bind _blackboard (`self.Blackboard`))
  (bind _orbitdirection (`self.OrbitDirection`))
  (bind _returnvalue (- (`self.ChangeOrbitDirectionTimer`) DeltaSeconds))
  (`parent.ReceiveTick` DeltaSeconds)
  (bind _asactor (cast `Actor` (`BlackboardComponent.GetValueAsObject` (`self.Blackboard`) (`self.Player`))))
  (`self.K2_SetFocus` _asactor)
  (set `self.ChangeOrbitDirectionTimer` _returnvalue)
  (if (< _returnvalue 0.0)
    (`BlackboardComponent.SetValueAsFloat` _blackboard _orbitdirection (* (`BlackboardComponent.GetValueAsFloat` _blackboard _orbitdirection) -1.0))
    (set `self.ChangeOrbitDirectionTimer` (`KismetMathLibrary.RandomFloatInRange` 1.0 3.0))))

(fn `UserConstructionScript`
  (`parent.UserConstructionScript`))