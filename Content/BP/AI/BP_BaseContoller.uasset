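; Base AI controller for BP_BaseEnemy pawns that alerts on perceiving the wizard and relays attack calls to the pawn.
; Stun events stop movement and refresh the Blackboard, which holds wander radius, sleep range and spawn location.
; Gated perception updates trigger Alert and a looping timer that reports "Noise" events at the pawn's location.
; Perceived "Noise" stimuli take the same alert path, so alerts can spread to nearby listeners.
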(event `self.ReceiveBeginPlay`
  (`self.K2_SetFocus` (`GameplayStatics.GetPlayerPawn` 0)))

(event `OnPawnBeginPlay`
  (bind _asbp_base_enemy (cast `/Game/BP/Enemies/BP_BaseEnemy` (`self.K2_GetPawn`))
    (:`then`
      (add `/Game/BP/Enemies/BP_BaseEnemy.Stunned_0` _asbp_base_enemy (delegate `OnStunned`))
      (add `/Game/BP/Enemies/BP_BaseEnemy.OnStunnedEnd_0` _asbp_base_enemy (delegate `StunnedEnd`)))
    (:`CastFailed`
      _))
  (`self.SetupBlackboard`))

(event `self.ReceiveTick`
  (params (DeltaSeconds :type "Float (single-precision)")))

(event `StunnedEnd`
  (`self.UpdateBlackboard` :!label _label))

(event `OnStunned`
  (`self.StopMovement`)
  (goto _label))

(event `self.AIPerception.OnPerceptionUpdated`
  (params (UpdatedActors :type "Array of Actor Object Reference (by ref)"))
  (`/Engine/EditorBlueprintResources/StandardMacros.Gate` false :!label _label_2
    (:`Exit`
      (for _array_element UpdatedActors
        (cast `/Game/BP/Wizards/BP_ComponentBasedWizard` _array_element)
        (`self.Alert` :!label _label_3)
        (if (`KismetSystemLibrary.K2_TimerExistsHandle` (`self.NoiseTimer`))
          (goto _label_2 :!via `Close`)
          (else
            (bind _returnvalue (`KismetSystemLibrary.K2_SetTimerDelegate` (delegate `AlertNearby`) 1.5 true))
            (set `self.NoiseTimer` _returnvalue)
            (goto _label_2 :!via `Close`)))))))

(event `AlertNearby`
  (`AISense_Hearing.ReportNoiseEvent` (`self.K2_GetActorLocation` (`self.K2_GetPawn`)) 1.0 self 0.0 "Noise"))

(event `self.AIPerception.OnTargetPerceptionUpdated`
  (params (Actor :type "Actor Object Reference") (Stimulus :type "AIStimulus Structure"))
  (if (== Stimulus_Tag "Noise")
    (goto _label_3)))

(fn `Alert`
  (locals (AlertedKey :type Name :default "Alerted"))
  (`self.UpdateBlackboard`)
  (if (not (`BlackboardComponent.GetValueAsBool` (`self.Blackboard`) (`local.AlertedKey`)))
    (`self.K2_SetFocus` (`GameplayStatics.GetPlayerPawn` 0))))

(fn `Attack`
  (bind _asbp_base_enemy (cast `/Game/BP/Enemies/BP_BaseEnemy` (`self.K2_GetPawn`)))
  (`/Game/BP/Enemies/BP_BaseEnemy.Attack` _asbp_base_enemy))

(fn `InitiateAttack`
  (`self.Attack`))

(fn `SetupBlackboard`
  (`self.UpdateBlackboard`)
  (`BlackboardComponent.SetValueAsVector` (`self.Blackboard`) (`self.SpawnLocation`) (`self.K2_GetActorLocation` (`self.K2_GetPawn`))))

(fn `UpdateBlackboard`
  (locals (Stunned :type Name :default "Stunned"))
  (bind _asbp_base_enemy (cast `/Game/BP/Enemies/BP_BaseEnemy` (`self.K2_GetPawn`))
    (:`then`
      _)
    (:`CastFailed`
      _))
  (`BlackboardComponent.SetValueAsFloat` (`self.Blackboard`) (`self.WanderRadius`) (`/Game/BP/Enemies/BP_BaseEnemy.WanderRadius` _asbp_base_enemy))
  (`BlackboardComponent.SetValueAsFloat` (`self.Blackboard`) (`self.SleepRangeKey`) (`self.SleepRange`)))

(fn `UserConstructionScript`)