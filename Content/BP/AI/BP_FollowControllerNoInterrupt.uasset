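; AI controller for a following enemy that runs the BP_FollowBehaviourNoInterrupt behavior tree on BeginPlay.
; It extends a parent controller, copying the player pawn and the controlled BP_BaseEnemy's attack range and timings into the Blackboard and setting an alerted flag on Alert.
; MoveToPlayer approaches the wizard character using the Blackboard attack range as acceptance radius.
; ChargeAttack forwards to the enemy pawn, while Attack defers to the parent.
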(event `self.ReceiveBeginPlay`
  (`parent.ReceiveBeginPlay`)
  (`self.RunBehaviorTree` "/Game/BP/AI/BP_FollowBehaviourNoInterrupt.BP_FollowBehaviourNoInterrupt"))

(fn `Alert`
  (`parent.Alert`)
  (`BlackboardComponent.SetValueAsBool` (`self.Blackboard`) (`self.Alerted_0`) true))

(fn `Attack`
  (`parent.Attack`))

(fn `Charge Attack`
  (bind _asbp_base_enemy (cast `/Game/BP/Enemies/BP_BaseEnemy` (`self.K2_GetPawn`)))
  (`/Game/BP/Enemies/BP_BaseEnemy.ChargeAttack` _asbp_base_enemy))

(fn `MoveToPlayer`
  (returns (result :type "EPathFollowingRequestResult Enum"))
  (bind _returnvalue (`self.MoveToActor` (`self.As BP Wizard Character 2`) (`BlackboardComponent.GetValueAsFloat` (`self.Blackboard`) (`self.AttackRange`)) true true true null))
  (return _returnvalue))

(fn `UpdateBlackboard`
  (bind _blackboard (`self.Blackboard`))
  (`parent.UpdateBlackboard`)
  (bind _asbp_base_enemy (cast `/Game/BP/Enemies/BP_BaseEnemy` (`self.K2_GetPawn`)))
  (if (`KismetSystemLibrary.IsValid` _blackboard)
    (`BlackboardComponent.SetValueAsObject` _blackboard (`self.Player`) (`GameplayStatics.GetPlayerPawn` 0))
    (`BlackboardComponent.SetValueAsFloat` _blackboard (`self.AttackRange`) (`/Game/BP/Enemies/BP_BaseEnemy.AttackRange` _asbp_base_enemy))
    (`BlackboardComponent.SetValueAsFloat` _blackboard (`self.AttackChargeTime`) (`/Game/BP/Enemies/BP_BaseEnemy.AttackChargeTime` _asbp_base_enemy))
    (`BlackboardComponent.SetValueAsFloat` _blackboard (`self.AttackRecoveryTime`) (`/Game/BP/Enemies/BP_BaseEnemy.AttackRecoveryTime` _asbp_base_enemy))))

(fn `UserConstructionScript`
  (`parent.UserConstructionScript`))