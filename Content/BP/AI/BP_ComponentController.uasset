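; BP_ComponentController is an AI controller for enemy pawns that attack and follow the player.
; It waits until both BeginPlay and Possess have fired, using two flags so setup works regardless of their order.
; It then runs the attack-follow behavior tree, focuses on player pawn 0, writes that pawn to a blackboard key, and calls OnControllerBeginPlay on the controlled BP_BaseEnemy.
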(event `self.ReceiveBeginPlay`
  (bind _returnvalue (`GameplayStatics.GetPlayerPawn` 0))
  (bind _output_get (set `self.HasBegunPlay` true))
  (if (and _output_get (stale `self.ReceivePossess` _output_get)) :!label _label
    (`self.RunBehaviorTree` "/Game/BP/AI/BP_ComponentAttackFollowController.BP_ComponentAttackFollowController")
    (`self.K2_SetFocus` _returnvalue)
    (`BlackboardComponent.SetValueAsObject` (`AIBlueprintHelperLibrary.GetBlackboard` null) (`self.Key Name`) _returnvalue)
    (bind _asbp_base_enemy (cast `/Game/BP/Enemies/BP_BaseEnemy` (`self.K2_GetPawn`)))
    (`/Game/BP/Enemies/BP_BaseEnemy.OnControllerBeginPlay` _asbp_base_enemy)))

(event `self.ReceivePossess`
  (params (PossessedPawn :type "Pawn Object Reference"))
  (bind _output_get (set `self.HasPossessed` true))
  (goto _label))

(fn `UserConstructionScript`)