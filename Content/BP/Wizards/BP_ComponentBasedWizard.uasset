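; Player wizard character built from components, with a HUD and mouse-aimed facing via a cursor-ray intersection with a horizontal plane.
; BindComponents injects dependencies into movement, dash, element casting, hit and trigger handling, hand animation, upgrade and camera components.
; Level-ups pause the game for an upgrade screen until completed.
; Fatal damage destroys the actor after a short delay if health is still depleted.
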(event `self.ReceiveBeginPlay`
  (bind _returnvalue (`|CreateWidget` "/Game/UI/BP_PlayerHUD.BP_PlayerHUD_C" (`GameplayStatics.GetPlayerController` 0)))
  (`/Game/UI/BP_PlayerHUD.Initialize` _returnvalue (`self.ExperienceComponent`))
  (`UserWidget.AddToViewport` _returnvalue 0))

(event `self.ReceiveTick`
  (params (DeltaSeconds :type "Float (single-precision)"))
  (`self.RotateTowardsMouse` DeltaSeconds))

(event `self.HealthManager.OnFatalDamageTakenDelegate`
  (params (DamagedComponent :type "BaseHealthComponent Object Reference") (Damage :type "Float (single-precision)") (OverkillDamage :type "Float (single-precision)") (DamageType :type "DamageType Object Reference") (InstigatedBy :type "Controller Object Reference") (DamageCauser :type "Actor Object Reference"))
  (`KismetSystemLibrary.Delay` 0.2)
  (if (`BaseHealthComponent.bIsDepleted` DamagedComponent)
    (`self.K2_DestroyActor`)))

(fn `BindComponents`
  (params (WizardController :type "/Game/BP/Wizards/WizardController Object Reference"))
  (bind _elementmanipulationcomponent (`self.ElementManipulationComponent`))
  (`/Engine/EditorBlueprintResources/StandardMacros.IsValid` WizardController
    (:`Is Valid`
      (`/Game/BP/Wizards/WizardController.Initialize` (`local.WizardController`) (`self.CharacterMovement`) (`self.DashComponent`) (`self.ElementManipulationComponent`) (`self.StatsComponent`))
      (`BaseDashComponent.Initialize` (`self.DashComponent`) (`self.CharacterMovement`) (`self.StatsComponent`))
      (`ElementManipulationComponent.Initialize` (`self.ElementManipulationComponent`) (`local.WizardController`) (`self.HandLeftSystem`) (`self.HandRightSystem`) (`self.StatsComponent`))
      (`HitHandlingComponent.Initialize` (`self.HitHandlingComponent`) (`|MakeArray` (`self.CapsuleComponent`) :!type "ShapeComponent Object Reference") (`self.AffiliationComponent`))
      (`BaseHealthComponent.BindHealthbar` (`self.BaseHealthComponent`) (`self.Healthbar`))
      (`TriggerHandlingComponent.Initialize` (`self.TriggerHandlingComponent`) (`self.ElementManipulationComponent`) (`self.HealthManager`))
      (set `ElementManipulationComponent.BasicAttackOriginPoint` (`self.BasicAttackOriginPointR`) _elementmanipulationcomponent)
      (set `ElementManipulationComponent.SpellOriginPoint` (`self.SpellOriginPoint`) _elementmanipulationcomponent)
      (set `SpringMovementMeshComponent.TargetLocation` (`self.HandLeftIdlePoint`) (`self.HandLeftSpring`))
      (set `SpringMovementMeshComponent.TargetLocation` (`self.HandRightIdlePoint`) (`self.HandRightSpring`))
      (`TiltToMovementComponent.Initialize` (`self.TiltToMovement`) (`self.Cube`) (`self.CharacterMovement`))
      (`WizardCastAnimator.Initialize` (`self.WizardCastAnimator`) (`self.ElementManipulationComponent`) (`self.HandLeftSpring`) (`self.HandRightSpring`) (`self.BasicAttackOriginPointL`) (`self.BasicAttackOriginPointR`) (`self.SpellOriginPoint`))
      (`SpellUpgradesComponent.Initialize` (`self.SpellUpgradesComponent`) (`self.ElementManipulationComponent`))
      (add `ExperienceComponent.OnLevelledUpDelegate` (`self.ExperienceComponent`) (`|CreateDelegate` :!event `OpenLevelUpScreen`))
      (`CameraControllerComponent.Initialize` (`self.CameraController`) (`self.SpringArm`) (`local.WizardController`)))))

(fn `OnLevelUpCompleted`
  (`Widget.RemoveFromParent` (`self.LevelUpUI`))
  (`GameplayStatics.SetGamePaused` false))

(fn `OpenLevelUpScreen`
  (params (ExperienceComponent :type "ExperienceComponent Object Reference") (NewLevel :type Integer))
  (locals (FirstElement :type "WizardElement Enum" :default "None") (SecondElementOptions :type "Array of WizardElement Enum") (SecondElement :type "WizardElement Enum" :default "None"))
  (`KismetSystemLibrary.PrintString` (`KismetStringLibrary.Conv_IntToString` NewLevel))
  (`/Engine/EditorBlueprintResources/StandardMacros.IsValid` (`self.LevelUpUI`)
    (:`Is Valid`
      _)
    (:`Is Not Valid`
      (bind _returnvalue (`|CreateWidget` "/Game/UI/NewLevelUpUi.NewLevelUpUi_C" (`GameplayStatics.GetPlayerController` 0)))
      (bind _output_get (set `self.LevelUpUI` _returnvalue))
      (add `/Game/UI/NewLevelUpUi.LeveledUp` _output_get (`|CreateDelegate` :!event `OnLevelUpCompleted`))
      (`/Game/UI/NewLevelUpUi.Cache Upgrade Component` _output_get (`self.CharacterUpgrades`))))
  (`UserWidget.AddToViewport` _output_get 0)
  (`GameplayStatics.SetGamePaused` true)
  (`/Game/UI/NewLevelUpUi.SetupElements` (`self.LevelUpUI`) (`self.ElementManipulationComponent`)))

(fn `RotateTowardsMouse`
  (params (DeltaTime :type "Float (double-precision)"))
  (bind _returnvalue (`self.K2_GetActorLocation`))
  (bind _mesh (`self.Mesh`))
  (bind (_worldlocation _worlddirection) (`PlayerController.DeprojectMousePositionToWorld` (`GameplayStatics.GetPlayerController` 0)))
  (`SceneComponent.K2_SetRelativeRotation` _mesh (`KismetMathLibrary.RInterpTo_Constant` (`SceneComponent.RelativeRotation` _mesh) (`KismetMathLibrary.FindLookAtRotation` _returnvalue (`.Intersection` (`KismetMathLibrary.LinePlaneIntersection_OriginNormal` _worldlocation (+ _worldlocation (* _worlddirection 10000.0)) _returnvalue (0.0 0.0 1.0)))) DeltaTime 1000.0) false false))

(fn `UserConstructionScript`)