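; Wizard player character Blueprint (an older component-based version) that wires up its movement, dash and element systems.
; On BeginPlay, BindComponents hands CharacterMovement, DashComponent and ElementManipulationComponent to the WizardController and passes controller and billboard references back.
; Tick updates the healthbar widget from the health ratio, and element and death events are forwarded.
; Level-up shows a widget and pauses the game until its LeveledUp callback resumes play.
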(event `self.ReceiveBeginPlay`
  (`self.BindComponents`))

(event `self.ReceiveTick`
  (params (DeltaSeconds :type "Float (single-precision)"))
  (bind _ashealthbar (cast `/Game/UI/Healthbar` (`WidgetComponent.GetWidget` (`self.Healthbar`))))
  (`/Game/UI/Healthbar.SetPercentage` _ashealthbar (/ (`self.GetHealth`) (`self.GetStartHealth`))))

(event `self.OnAddElement`
  (`self.ElementAdded`))

(event `self.OnDeathEvent`
  (`self.Death`))

(event `self.OnLevelUp`
  (`/Engine/EditorBlueprintResources/StandardMacros.IsValid` (`self.LevelUpUi`)
    (:`Is Valid`
      _)
    (:`Is Not Valid`
      (bind _returnvalue (`|CreateWidget` "/Game/UI/LevelUpUi.LevelUpUi_C"))
      (bind _output_get (set `self.LevelUpUi` _returnvalue))))
  (add `/Game/UI/LevelUpUi.LeveledUp` _output_get (delegate `LeveledUp`))
  (`UserWidget.AddToViewport` _output_get 0)
  (`GameplayStatics.SetGamePaused` true))

(event `LeveledUp`
  (`GameplayStatics.SetGamePaused` false)
  (`Widget.RemoveFromParent` (`self.LevelUpUi`)))

(fn `BindComponents`
  (locals (WizardController :type "/Game/BP/Wizards/WizardController Object Reference"))
  (bind _wizardcontroller (`local.WizardController`))
  (bind _dashcomponent (`self.DashComponent`))
  (bind _elementmanipulationcomponent (`self.ElementManipulationComponent`))
  (bind _wizardcontroller_2 (`local.WizardController`))
  (bind _aswizard_controller (cast `/Game/BP/Wizards/WizardController` (`self.GetController`)))
  (set `local.WizardController` _aswizard_controller)
  (set `/Game/BP/Wizards/WizardController.MovementComponent` (`self.CharacterMovement`) _wizardcontroller_2)
  (set `/Game/BP/Wizards/WizardController.DashComponent` _dashcomponent _wizardcontroller_2)
  (set `BaseDashComponent.CharacterMovementComponent` (`self.CharacterMovement`) _dashcomponent)
  (set `/Game/BP/Wizards/WizardController.ElementManipulationComponent` _elementmanipulationcomponent _wizardcontroller)
  (set `ElementManipulationComponent.Controller` _wizardcontroller _elementmanipulationcomponent)
  (set `ElementManipulationComponent.FirstElementBillboard` (`self.FirstElementBillboard`) _elementmanipulationcomponent)
  (set `ElementManipulationComponent.SecondElementBillboard` (`self.SecondElementBillboard`) _elementmanipulationcomponent))

(fn `UserConstructionScript`)