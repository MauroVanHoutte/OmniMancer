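; BP_WizardCharacter is a wizard character Blueprint that presents its health bar and level-up screen.
; Tick sets the Healthbar widget component's percentage from current over starting health.
; On level-up it creates or reuses the level-up widget, shows it and pauses the game until that widget's LeveledUp event resumes play and removes it.
; Element-added and death events are forwarded to CallElementAdded and CallDeath.
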(event `self.ReceiveTick`
  (params (DeltaSeconds :type "Float (single-precision)"))
  (bind _ashealthbar (cast `/Game/UI/Healthbar` (`WidgetComponent.GetWidget` (`self.Healthbar`))))
  (bind _returnvalue (`self.GetHealth`))
  (bind _returnvalue_2 (`self.GetStartHealth`))
  (`/Game/UI/Healthbar.SetPercentage` _ashealthbar (/ _returnvalue _returnvalue_2)))

(event `self.OnAddElement`
  (`self.ElementAdded`))

(event `self.OnDeathEvent`
  (`self.Death`))

(event `self.OnLevelUp`
  (`/Engine/EditorBlueprintResources/StandardMacros.IsValid` (`self.LevelUpUi`)
    (:`Is Valid`
      _)
    (:`Is Not Valid`
      (bind _returnvalue (`|CreateWidget` "/Game/UI/LevelUpUi.LevelUpUi_C"))
      (bind _output_get (set `self.LevelUpUi` _returnvalue))))
  (add `/Game/UI/LevelUpUi.LeveledUp` _output_get (delegate `LeveledUp`))
  (`UserWidget.AddToViewport` _output_get 0)
  (`GameplayStatics.SetGamePaused` true))

(event `LeveledUp`
  (`GameplayStatics.SetGamePaused` false)
  (`Widget.RemoveFromParent` (`self.LevelUpUi`)))

(fn `UserConstructionScript`)