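; Player controller for the wizard character that maps Enhanced Input actions to gameplay components and shows the mouse cursor.
; On possess it passes itself to the wizard's BindComponents, with Initialize storing movement, dash, element-manipulation and stat component references.
; Input forwards movement, dash, Fire/Frost/Wind element selection, and pressed/held/released attack and cast events to those components.
; It also broadcasts interaction, toggles a lazily created pause menu, and has a debug key destroying all enemies.
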(event Input|EnhancedActionEvents|EnhancedInputActionMovementAction
  (params (ActionValue :type Vector%202D%20Structure) (ElapsedSeconds :type Float%20%28double-precision%29) (TriggeredSeconds :type Float%20%28double-precision%29) (InputAction :type Input%20Action%20Object%20Reference :default "/Game/BP/Wizards/Input/Actions/MovementAction.MovementAction"))
  (bind _movementcomponent (Variables|Default|GetMovementComponent))
  (Utilities|IsValid _movementcomponent
    (:Is%20Valid
      (Class|PawnMovementComponent|AddInputVector _movementcomponent (Math|Conversions|ToVector(Vector2D) ActionValue) false))))

(event Input|EnhancedActionEvents|EnhancedInputActionDashAction
  (params (ActionValue :type Boolean) (ElapsedSeconds :type Float%20%28double-precision%29) (TriggeredSeconds :type Float%20%28double-precision%29) (InputAction :type Input%20Action%20Object%20Reference :default "/Game/BP/Wizards/Input/Actions/DashAction.DashAction"))
  (bind _dashcomponent (Variables|Default|GetDashComponent))
  (Utilities|IsValid _dashcomponent
    (:Is%20Valid
      (Class|BaseDashComponent|TryExecuteDash _dashcomponent))))

(event Input|EnhancedActionEvents|EnhancedInputActionBaseAttackPressed
  (params (ActionValue :type Boolean) (ElapsedSeconds :type Float%20%28double-precision%29) (TriggeredSeconds :type Float%20%28double-precision%29) (InputAction :type Input%20Action%20Object%20Reference :default "/Game/BP/Wizards/Input/Actions/BaseAttackPressed.BaseAttackPressed"))
  (bind _elementmanipulationcomponent (Variables|Default|GetElementManipulationComponent))
  (Utilities|IsValid _elementmanipulationcomponent
    (:Is%20Valid
      (Class|ElementManipulationComponent|HandleBasicAttackInputPressed _elementmanipulationcomponent))))

(event Input|EnhancedActionEvents|EnhancedInputActionBaseAttackReleased
  (params (ActionValue :type Boolean) (ElapsedSeconds :type Float%20%28double-precision%29) (TriggeredSeconds :type Float%20%28double-precision%29) (InputAction :type Input%20Action%20Object%20Reference :default "/Game/BP/Wizards/Input/Actions/BaseAttackReleased.BaseAttackReleased"))
  (bind _elementmanipulationcomponent (Variables|Default|GetElementManipulationComponent))
  (Utilities|IsValid _elementmanipulationcomponent
    (:Is%20Valid
      (Class|ElementManipulationComponent|HandleBasicAttackInputReleased _elementmanipulationcomponent))))

(event Input|EnhancedActionEvents|EnhancedInputActionSpellCastPressed
  (params (ActionValue :type Boolean) (ElapsedSeconds :type Float%20%28double-precision%29) (TriggeredSeconds :type Float%20%28double-precision%29) (InputAction :type Input%20Action%20Object%20Reference :default "/Game/BP/Wizards/Input/Actions/SpellCastPressed.SpellCastPressed"))
  (bind _elementmanipulationcomponent (Variables|Default|GetElementManipulationComponent))
  (Utilities|IsValid _elementmanipulationcomponent
    (:Is%20Valid
      (Class|ElementManipulationComponent|HandleCastInputPressed _elementmanipulationcomponent))))

(event Input|EnhancedActionEvents|EnhancedInputActionSpellCastReleased
  (params (ActionValue :type Boolean) (ElapsedSeconds :type Float%20%28double-precision%29) (TriggeredSeconds :type Float%20%28double-precision%29) (InputAction :type Input%20Action%20Object%20Reference :default "/Game/BP/Wizards/Input/Actions/SpellCastReleased.SpellCastReleased"))
  (bind _elementmanipulationcomponent (Variables|Default|GetElementManipulationComponent))
  (Utilities|IsValid _elementmanipulationcomponent
    (:Is%20Valid
      (Class|ElementManipulationComponent|HandleCastInputReleased _elementmanipulationcomponent))))

(event Input|EnhancedActionEvents|EnhancedInputActionSpellCastDown
  (params (ActionValue :type Boolean) (ElapsedSeconds :type Float%20%28double-precision%29) (TriggeredSeconds :type Float%20%28double-precision%29) (InputAction :type Input%20Action%20Object%20Reference :default "/Game/BP/Wizards/Input/Actions/SpellCastDown.SpellCastDown"))
  (bind _elementmanipulationcomponent (Variables|Default|GetElementManipulationComponent))
  (Utilities|IsValid _elementmanipulationcomponent
    (:Is%20Valid
      (Class|ElementManipulationComponent|HandleCastInputDown _elementmanipulationcomponent))))

(event Input|EnhancedActionEvents|EnhancedInputActionFireElementAction
  (params (ActionValue :type Boolean) (ElapsedSeconds :type Float%20%28double-precision%29) (TriggeredSeconds :type Float%20%28double-precision%29) (InputAction :type Input%20Action%20Object%20Reference :default "/Game/BP/Wizards/Input/Actions/FireElementAction.FireElementAction"))
  (bind _elementmanipulationcomponent (Variables|Default|GetElementManipulationComponent))
  (Utilities|IsValid _elementmanipulationcomponent
    (:Is%20Valid
      (Class|ElementManipulationComponent|AddElement _elementmanipulationcomponent "Fire"))))

(event Input|EnhancedActionEvents|EnhancedInputActionFrostElementAction
  (params (ActionValue :type Boolean) (ElapsedSeconds :type Float%20%28double-precision%29) (TriggeredSeconds :type Float%20%28double-precision%29) (InputAction :type Input%20Action%20Object%20Reference :default "/Game/BP/Wizards/Input/Actions/FrostElementAction.FrostElementAction"))
  (bind _elementmanipulationcomponent (Variables|Default|GetElementManipulationComponent))
  (Utilities|IsValid _elementmanipulationcomponent
    (:Is%20Valid
      (Class|ElementManipulationComponent|AddElement _elementmanipulationcomponent "Frost"))))

(event Input|EnhancedActionEvents|EnhancedInputActionWindElementAction
  (params (ActionValue :type Boolean) (ElapsedSeconds :type Float%20%28double-precision%29) (TriggeredSeconds :type Float%20%28double-precision%29) (InputAction :type Input%20Action%20Object%20Reference :default "/Game/BP/Wizards/Input/Actions/WindElementAction.WindElementAction"))
  (bind _elementmanipulationcomponent (Variables|Default|GetElementManipulationComponent))
  (Utilities|IsValid _elementmanipulationcomponent
    (:Is%20Valid
      (Class|ElementManipulationComponent|AddElement _elementmanipulationcomponent "Wind"))))

(event Input|EnhancedActionEvents|EnhancedInputActionInteractAction
  (params (ActionValue :type Boolean) (ElapsedSeconds :type Float%20%28double-precision%29) (TriggeredSeconds :type Float%20%28double-precision%29) (InputAction :type Input%20Action%20Object%20Reference :default "/Game/BP/Wizards/Input/Actions/InteractAction.InteractAction"))
  (Class|WizardController|BroadcastInteractDelegate))

(event Input|EnhancedActionEvents|EnhancedInputActionPauseAction
  (params (ActionValue :type Boolean) (ElapsedSeconds :type Float%20%28double-precision%29) (TriggeredSeconds :type Float%20%28double-precision%29) (InputAction :type Input%20Action%20Object%20Reference :default "/Game/BP/Wizards/Input/Actions/PauseAction.PauseAction"))
  (Variables|Default|GetPauseMenu
    (:then
      (if (Widget|IsVisible (stale _output_get))
        (Game|SetGamePaused false)
        (Widget|SetVisibility (Variables|Default|GetPauseMenu) "Collapsed")
        (else
          (Game|SetGamePaused true :!label _label)
          (Widget|SetVisibility (Variables|Default|GetPauseMenu) "Visible"))))
    (:else
      (bind _returnvalue (UserInterface|CreateWidget "/Game/UI/BP_PauseMenu.BP_PauseMenu_C" self))
      (bind _output_get (Variables|Default|SetPauseMenu _returnvalue))
      (UserInterface|Viewport|AddtoPlayerScreen _output_get)
      (goto _label))))

(event Input|EnhancedActionEvents|EnhancedInputActionBaseAttackDown
  (params (ActionValue :type Boolean) (ElapsedSeconds :type Float%20%28double-precision%29) (TriggeredSeconds :type Float%20%28double-precision%29) (InputAction :type Input%20Action%20Object%20Reference :default "/Game/BP/Wizards/Input/Actions/BaseAttackDown.BaseAttackDown"))
  (bind _elementmanipulationcomponent (Variables|Default|GetElementManipulationComponent))
  (Utilities|IsValid _elementmanipulationcomponent
    (:Is%20Valid
      (Class|ElementManipulationComponent|HandleBasicAttackInputDown _elementmanipulationcomponent))))

(event EventBeginPlay
  (Input|AddMappingContext (PlayerController|LocalPlayerSubsystems|GetEnhancedInputLocalPlayerSubsystem self) "/Game/BP/Wizards/Input/NewInputMappingContext.NewInputMappingContext" 0 "(bIgnoreAllPressedKeysUntilRelease=True,bForceImmediately=False,bNotifyUserSettings=False)")
  (Variables|Default|SetbShowMouseCursor true))

(event EventPossess
  (params (PossessedPawn :type Pawn%20Object%20Reference))
  (bind _asbp_component_based_wizard (Utilities|Casting|CastToBP_ComponentBasedWizard PossessedPawn))
  (Default|BindComponents _asbp_component_based_wizard self))

(event Input|KeyboardEvents|DebugKeyL
  (params (Key :type Key%20Structure :default "None") (ActionValue :type Input%20Action%20Value%20Structure))
  (:Pressed
    (bind _outactors (Actor|GetAllActorsOfClass "/Game/BP/Enemies/BP_BaseEnemy.BP_BaseEnemy_C"))
    (for _array_element _outactors
      (Actor|DestroyActor _array_element))))

(fn ConstructionScript)

(fn Initialize
  (params (CharacterMovementComp :type Character%20Movement%20Component%20Object%20Reference) (DashComponent :type Base%20Dash%20Component%20Object%20Reference) (ElementManipulationComp :type Element%20Manipulation%20Component%20Object%20Reference) (StatComponent :type Stat%20Component%20Object%20Reference))
  (Variables|Default|SetMovementComponent CharacterMovementComp)
  (Variables|Default|SetDashComponent DashComponent)
  (Variables|Default|SetElementManipulationComponent ElementManipulationComp)
  (Variables|Default|SetPawnStats StatComponent))