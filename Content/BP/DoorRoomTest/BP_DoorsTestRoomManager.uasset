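; Test-room manager that runs a wave-based combat encounter when the wizard character enters its box.
; Entry closes all TestDoors, animates roof material opacity and, after a delay, starts a looping wave timer.
; Each wave picks random enemy types and navmesh group locations, shows debug-sphere warnings and queues the spawns behind a timer.
; Spawned enemies are tracked until destroyed; doors reopen once none remain and the wave timer has ended.
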(event `self.ReceiveBeginPlay`
  (bind _returnvalue (`PrimitiveComponent.CreateDynamicMaterialInstance` (`self.Cube`) 0 "/Game/Materials/M_RoomRoof.M_RoomRoof" "None"))
  (set `self.RoofMaterial` _returnvalue))

(event `self.ReceiveTick`
  (params (DeltaSeconds :type "Float (single-precision)")))

(event `self.Box.OnComponentBeginOverlap`
  (params (OverlappedComponent :type "PrimitiveComponent Object Reference") (OtherActor :type "Actor Object Reference") (OtherComp :type "PrimitiveComponent Object Reference") (OtherBodyIndex :type Integer) (bFromSweep :type Boolean) (SweepResult :type "HitResult Structure (by ref)"))
  (if (not (`self.RoomStarted`))
    (cast `/Game/BP/Wizards/BP_ComponentBasedWizard` OtherActor)
    (`|ExecutionSequence`
      (:`then_0`
        (set `self.RoomStarted` true)
        (`KismetSystemLibrary.Delay` 5.0)
        (`self.StartSpawning`))
      (:`then_1`
        (bind _outactors (`GameplayStatics.GetAllActorsOfClass` "/Game/BP/DoorRoomTest/TestDoor.TestDoor_C"))
        (for _array_element _outactors
          (`/Game/BP/DoorRoomTest/TestDoor.Close` _array_element)))
      (:`then_2`
        (bind (_direction _newtrack_0) (`Timeline|Timeline`)
          (:`Update`
            (`MaterialInstanceDynamic.SetScalarParameterValue` (`self.RoofMaterial`) "Opacity" _newtrack_0)))))))

(event `StartSpawning`
  (`self.StartWave`)
  (bind _returnvalue (`KismetSystemLibrary.K2_SetTimerDelegate` (`|CreateDelegate` :!event `StartWave`) (`self.TimeBetweenWaves`) true))
  (set `self.WaveTImerHandle` _returnvalue))

(event `StartWave`
  (`/Engine/EditorBlueprintResources/StandardMacros.IncrementInt` (`self.CurrentWave`)
    (:`  `
      (if (> (`self.CurrentWave`) (`self.Waves`))
        (`KismetSystemLibrary.K2_ClearAndInvalidateTimerHandle` (`self.WaveTImerHandle`))
        (else
          (`self.SpawnWaveEnemies`))))))

(fn `HandleEnemyDestroyed`
  (params (DestroyedActor :type "Actor Object Reference"))
  (bind _aliveenemies (`self.AliveEnemies`))
  (remove `self.OnDestroyed` (`|CreateDelegate` :!event `HandleEnemyDestroyed`))
  (`KismetArrayLibrary.Array_RemoveItem` _aliveenemies DestroyedActor)
  (if (and (`KismetArrayLibrary.Array_IsEmpty` _aliveenemies) (not (`KismetSystemLibrary.K2_IsValidTimerHandle` (`self.WaveTImerHandle`))))
    (bind _outactors (`GameplayStatics.GetAllActorsOfClass` "/Game/BP/DoorRoomTest/TestDoor.TestDoor_C"))
    (for _array_element _outactors
      (`/Game/BP/DoorRoomTest/TestDoor.Open` _array_element))))

(fn `SpawnQueuedEnemies`
  (for _array_element (`self.EnemiesToSpawn`)
    (for _array_element_2 (`.Locations_10_223AA8BC4B4B42BC7A7156927DF1BA2C` (break `/Game/BP/DoorRoomTest/EnemySpawn` _array_element))
      (bind _returnvalue (`|SpawnActorFromClass` (break `/Game/BP/DoorRoomTest/EnemySpawn` _array_element) (`KismetMathLibrary.MakeTransform` _array_element_2) "AdjustIfPossibleButAlwaysSpawn" "MultiplyWithRoot" null null))
      (`KismetArrayLibrary.Array_Add` (`self.AliveEnemies`) _returnvalue)
      (add `self.OnDestroyed` _returnvalue (`|CreateDelegate` :!event `HandleEnemyDestroyed`))))
  (`KismetArrayLibrary.Array_Clear` (`self.EnemiesToSpawn`)))

(fn `SpawnWaveEnemies`
  (locals (SelectedEnemyType :type "Actor Class Reference") (GroupCenter :type "Vector Structure" :default (0.0 0.0 0.0)) (SpawnLocations :type "Array of Vector Structure"))
  (bind _spawnlocations (`local.SpawnLocations`))
  (bind (_origin _boxextent) (`KismetSystemLibrary.GetComponentBounds` (`self.Box`)))
  ;[1 1 1] Spawn Groups
  (for _ (range 1 (+ (`self.GroupsPerWave`) 1))
    (bind _keys (`BlueprintMapLibrary.Map_Keys` (`self.TypeGroupSizes`)))
    (bind _output_get (set `local.SelectedEnemyType` (`KismetArrayLibrary.Array_Random` _keys)))
    (set `local.GroupCenter` (`NavigationSystemV1.K2_ProjectPointToNavigation` (`NavigationSystemV1.GetNavigationSystem`) (`NavigationSystemV1.K2_ProjectPointToNavigation` (`KismetMathLibrary.RandomPointInBoundingBox` _origin _boxextent)) null null (1000.0 1000.0 1000.0)))
    (for _ (range 1 (+ (`BlueprintMapLibrary.Map_Find` (`self.TypeGroupSizes`) _output_get) 1))
      (bind _returnvalue (`KismetArrayLibrary.Array_Add` _spawnlocations (`KismetMathLibrary.MakeVector` (.x (`NavigationSystemV1.K2_GetRandomReachablePointInRadius` (`NavigationSystemV1.GetNavigationSystem`) (`local.GroupCenter`) (`self.GroupRadius`) null null)) (.y (`NavigationSystemV1.K2_GetRandomReachablePointInRadius` (`NavigationSystemV1.GetNavigationSystem`) (`local.GroupCenter`) (`self.GroupRadius`) null null)) (+ (.z (`NavigationSystemV1.K2_GetRandomReachablePointInRadius` (`NavigationSystemV1.GetNavigationSystem`) (`local.GroupCenter`) (`self.GroupRadius`) null null)) 50.0))))
      (`KismetSystemLibrary.DrawDebugSphere` (`|GetArrayItem` _spawnlocations _returnvalue) 100.0 12 (struct :`R` 1.0 :`B` 0.048188 :`A` 1.0) (`self.SpawnWarningTIme`) 1.0))
    (`KismetArrayLibrary.Array_Add` (`self.EnemiesToSpawn`) (make `/Game/BP/DoorRoomTest/EnemySpawn` (`local.SelectedEnemyType`) (`local.SpawnLocations`)))
    (`KismetArrayLibrary.Array_Clear` (`local.SpawnLocations`)))
  (`KismetSystemLibrary.K2_SetTimerDelegate` (`|CreateDelegate` :!event `SpawnQueuedEnemies`) (`self.SpawnWarningTIme`)))

(fn `UserConstructionScript`)