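; BP_SpawnLocation is an enemy spawn marker that shows a spinning decal until its enemy spawns.
; BeginPlay gives the decal a random starting roll, and Tick keeps rolling it at DecalSpinSpeed scaled by delta time.
; It binds to OnEnemySpawnedDelegate, whose handler hands the marker to the actor pooling subsystem to be returned to the pool or destroyed.
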(event `self.ReceiveBeginPlay`
  (bind _decal (`self.Decal`))
  (bind (_relativerotation_roll _relativerotation_pitch _relativerotation_yaw) (`KismetMathLibrary.BreakRotator` (`SceneComponent.RelativeRotation` _decal)))
  (`SceneComponent.K2_SetRelativeRotation` _decal (`KismetMathLibrary.MakeRotator` (`KismetMathLibrary.RandomFloatInRange` 0.0 360.0) _relativerotation_pitch _relativerotation_yaw) false false)
  (add `self.OnEnemySpawnedDelegate` (delegate `OnEnemySpawnedDelegate_Event`)))

(event `OnEnemySpawnedDelegate_Event` :!signature `self.OnEnemySpawnedDelegate`
  (params (SpawnedEnemy :type "Actor Object Reference"))
  (`ActorPoolingSubsystem.ReturnActorToPoolOrDestroy` (subsystem `ActorPoolingSubsystem`) self))

(event `self.ReceiveTick`
  (params (DeltaSeconds :type "Float (single-precision)"))
  (`SceneComponent.K2_AddRelativeRotation` (`self.Decal`) (`KismetMathLibrary.MakeRotator` (* DeltaSeconds (`self.Decal Spin Speed`))) false false))

(fn `UserConstructionScript`)