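; BP_RoomManager runs a room's combat encounter and shop, building on encounter logic defined outside this Blueprint.
; The player pawn leaving ActivationCollider starts the encounter once, with separate events starting the boss or enemy-wave encounter manager.
; Both managers' completion delegates feed a shared OnEncounterCompleted call.
; OpenShop extends the parent behavior by opening the Shop reference when it is valid.
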(event `self.ReceiveBeginPlay`)

(event `self.ReceiveTick`
  (params (DeltaSeconds :type "Float (single-precision)")))

(event `self.StartBossEncounter`
  (`BaseCombatEncounterManager.StartEncounter` (`self.BossCombatEncounterManager`)))

(event `self.StartEnemyWavesEncounter`
  (`BaseCombatEncounterManager.StartEncounter` (`self.WaveCombatEncounterManager`)))

(event `self.WaveCombatEncounterManager.OnEncounterCompletedDelegate`
  (`self.OnEncounterCompleted` :!label _label))

(event `self.BossCombatEncounterManager.OnEncounterCompletedDelegate`
  (goto _label))

(event `self.ActivationCollider.OnComponentEndOverlap`
  (params (OverlappedComponent :type "PrimitiveComponent Object Reference") (OtherActor :type "Actor Object Reference") (OtherComp :type "PrimitiveComponent Object Reference") (OtherBodyIndex :type Integer))
  (if (and (== OtherActor (`GameplayStatics.GetPlayerPawn` 0)) (not (`self.HasEncounterStarted`)))
    (`self.StartEncounter`)))

(event `self.OpenShop`
  (`parent.OpenShop`)
  (if (`KismetSystemLibrary.IsValid` (`self.Shop`))
    (`/Game/BP/Shop/BP_Shop.OpenShop` (`self.Shop`))))

(fn `UserConstructionScript`)