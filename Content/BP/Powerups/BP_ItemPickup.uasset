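; BP_ItemPickup is a pooled item pickup actor with a floating, rotating mesh and a widget component.
; A tick after BeginPlay, a valid TestItem is applied through SetItem and the ItemWidget's description is hidden.
; The description is also hidden whenever the actor is taken from the pool.
; Tick bobs the mesh on a sine wave around a base height and spins it in yaw.
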(event `self.ReceiveBeginPlay`
  (bind _testitem (`self.TestItem`))
  (`KismetSystemLibrary.DelayUntilNextTick`)
  (`/Engine/EditorBlueprintResources/StandardMacros.IsValid` _testitem
    (:`Is Valid`
      (`self.SetItem` _testitem)
      (bind _asitem_widget (cast `ItemWidget` (`WidgetComponent.GetUserWidgetObject` (`self.Widget`))))
      (`ItemWidget.HideDescription` _asitem_widget))))

(event `PooledActorInterface.OnActorTakenFromPool`
  (bind _asitem_widget (cast `ItemWidget` (`WidgetComponent.GetUserWidgetObject` (`self.Widget`))))
  (`ItemWidget.HideDescription` _asitem_widget))

(event `self.ReceiveTick`
  (params (DeltaSeconds :type "Float (single-precision)"))
  (bind _meshcomponent (`self.MeshComponent`))
  (bind (_relativelocation_x _relativelocation_y) (`KismetMathLibrary.BreakVector` (`SceneComponent.RelativeLocation` _meshcomponent)))
  (set `self.Time` (+ (`self.Time`) DeltaSeconds))
  (`SceneComponent.K2_SetRelativeLocation` _meshcomponent (`KismetMathLibrary.MakeVector` _relativelocation_x _relativelocation_y (+ (* (`KismetMathLibrary.Sin` (* (`self.Time`) (`self.BobbingFrequency`))) (`self.BobbingOffset`)) (`self.BaseHeight`))) false false)
  (`SceneComponent.K2_AddLocalRotation` _meshcomponent (`KismetMathLibrary.MakeRotator` 0.0 0.0 (* DeltaSeconds (`self.RotationSpeed`))) false false))

(fn `UserConstructionScript`)