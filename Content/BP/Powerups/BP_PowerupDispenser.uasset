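; BP_PowerupDispenser is a dispenser actor that spawns power-ups when a WizardCharacter overlaps it.
; While its Uses counter is nonzero, each overlap decrements it, spawns a BP_PowerUp 300 units above the dispenser and passes it the configured PowerUpEffect.
; On BeginPlay it writes its Text variable to a text render component as a label.
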(event `self.ReceiveBeginPlay`
  (`TextRenderComponent.K2_SetText` (`self.TextRender`) (`KismetTextLibrary.Conv_StringToText` (`self.Text`))))

(event `self.ReceiveActorBeginOverlap`
  (params (OtherActor :type "Actor Object Reference"))
  (cast `WizardCharacter` OtherActor)
  (if (!= (`self.Uses`) 0)
    (`/Engine/EditorBlueprintResources/StandardMacros.DecrementInt` (`self.Uses`)
      (:`  `
        (bind _returnvalue (`|SpawnActorFromClass` "/Game/BP/Powerups/BP_PowerUp.BP_PowerUp_C" (`KismetMathLibrary.MakeTransform` (+ (`self.K2_GetActorLocation`) (0.0 0.0 300.0))) "Undefined" "OverrideRootScale" null null))
        (`PowerUp.SetEffect` _returnvalue (`self.PowerUpEffect`))))))

(fn `UserConstructionScript`)