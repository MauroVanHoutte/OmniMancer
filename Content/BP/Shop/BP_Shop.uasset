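; BP_Shop is a shop actor that, on OpenShop, tosses three random item pickups out to three target locations.
; OpenShop copies the item list and calls SpawnItem per target, removing each chosen item from the copy to avoid repeat picks.
; SpawnItem takes a BP_ItemPickup from the actor pool, places it at the spawn point and launches its projectile movement along a suggested high arc.
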(event `OpenShop`
  (set `self.UnusedItems` (`ItemList.Items` (`self.Items`)))
  (`|ExecutionSequence`
    (:`then_0`
      (`self.SpawnItem` (`SceneComponent.K2_GetComponentLocation` (`self.ItemTargetLocation1`))))
    (:`then_1`
      (`self.SpawnItem` (`SceneComponent.K2_GetComponentLocation` (`self.ItemTargetLocation2`))))
    (:`then_2`
      (`self.SpawnItem` (`SceneComponent.K2_GetComponentLocation` (`self.ItemTargetLocation3`))))))

(fn `SpawnItem`
  (params (TargetLocation :type "Vector Structure"))
  (locals (TempItemVariable :type "ItemConfig Object Reference"))
  (bind _returnvalue (`ActorPoolingSubsystem.GetActorFromPool` (subsystem `ActorPoolingSubsystem`) "/Game/BP/Powerups/BP_ItemPickup.BP_ItemPickup_C"))
  (bind _asbp_item_pickup (cast `/Game/BP/Powerups/BP_ItemPickup` _returnvalue))
  (bind _output_get (set `local.TempItemVariable` (`KismetArrayLibrary.Array_Random` (`self.UnusedItems`))))
  (`ItemPickup.SetItem` _asbp_item_pickup _output_get)
  (`KismetArrayLibrary.Array_RemoveItem` (`self.UnusedItems`) (`local.TempItemVariable`))
  (`self.K2_SetActorLocation` _asbp_item_pickup (`SceneComponent.K2_GetComponentLocation` (`self.ItemSpawnPoint`)) false false)
  (bind _tossvelocity (`GameplayStatics.BlueprintSuggestProjectileVelocity` (`SceneComponent.K2_GetComponentLocation` (`self.ItemSpawnPoint`)) (`local.TargetLocation`) 650.0 0.0 "DoNotTrace" 0.0 true))
  (`ProjectileMovementComponent.SetVelocityInLocalSpace` (`/Game/BP/Powerups/BP_ItemPickup.ProjectileMovement` _asbp_item_pickup) _tossvelocity))

(fn `UserConstructionScript`)